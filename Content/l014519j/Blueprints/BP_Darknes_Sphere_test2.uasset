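; Darkness sphere actor that acts as a safe zone, damaging the player outside it.
; Ending overlap starts a looping timer that damages the player character and a slow camera and audio fade-out.
; Beginning overlap clears that timer and stops the fade.
; At BeginPlay a one-shot timer uses seconds from a game mode interface, then collapses the sphere's radius to zero in one step.
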(event OnComponentEndOverlap(CollisionComponent)
  (params (OverlappedComponent :type Primitive%20Component%20Object%20Reference) (OtherActor :type Actor%20Object%20Reference) (OtherComp :type Primitive%20Component%20Object%20Reference) (OtherBodyIndex :type Integer))
  ;[1 1 1] Starts Darkness Damage on timer when outside sphere - l014519j
  (bind _returnvalue (Utilities|Time|SetTimerbyEvent (delegate Custom|Update) 2.0 true 2.0))
  (Variables|Default|SetHealth _returnvalue)
  (CameraFades|StartCameraFade :self (Game|GetPlayerCameraManager 0) :ToAlpha 1.0 :Duration 2e+01 :bShouldFadeAudio true :bHoldWhenFinished true))

(event Custom|Update
  ;[1 1 1] Starts Darkness Damage on timer when outside sphere - l014519j
  (Class|BPIDamage|TakeDamage(Message) (Game|GetPlayerCharacter 0) 1e+01))

(event Custom|Scale%20Update
  ;[1 1 1] Shrinks Darkness Sphere based on Game Timer - l014519j
  (Components|Sphere|SetSphereRadius (Variables|Default|GetSphere%20Collision) 0.0 true))

(event EventBeginPlay
  ;[1 1 1] Shrinks Darkness Sphere based on Game Timer - l014519j
  (bind _assphere_collision (Utilities|Casting|CastToSphereComponent (Variables|Default|GetCollisionComponent)))
  (Variables|Default|SetSphere%20Collision _assphere_collision)
  (bind _sec (Class|BPISec|IGetSec(Message) (Game|GetGameMode)))
  (bind _returnvalue (Utilities|Time|SetTimerbyEvent (delegate Custom|Scale%20Update) (Math|Conversions|ToFloat(Integer) _sec)))
  (Variables|Default|SetDarkness_Scale _returnvalue))

(event Collision|EventActorBeginOverlap
  (params (OtherActor :type Actor%20Object%20Reference))
  ;[1 1 1] Stops Damage When in Sphere - l014519j
  (Utilities|Time|ClearandInvalidateTimerbyHandle (Variables|Default|GetHealth))
  (CameraFades|StopCameraFade (Game|GetPlayerCameraManager 0)))

(fn ConstructionScript)