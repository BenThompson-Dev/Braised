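; Character Blueprint that runs a minutes-and-seconds countdown and opens test_level01 when time runs out.
; Tick feeds a one-second Delay, so Sec and Min step down about once per second.
; BeginPlay adds two timer widgets, DSBP_Timer and W_Timer_Int, to the viewport.
; A disconnected count-up timer using TimeSec and TimeMin remains in the event graph and never runs.
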(event EventTick
  (params (DeltaSeconds :type Float%20%28single-precision%29))
  (Utilities|FlowControl|Delay 1.0)
  (if (== (Variables|Default|GetSec) 0)
    (if (== (Variables|Default|GetMin) 0)
      (Game|OpenLevel(byName) "test_level01")
      (else
        (Variables|Default|SetSec 59)
        (Variables|Default|SetMin (- (Variables|Default|GetMin) 1))))
    (else
      (Variables|Default|SetSec (- (Variables|Default|GetSec) 1)))))

(event EventBeginPlay
  (Utilities|FlowControl|Sequence
    (:then_0
      (bind _returnvalue (UserInterface|CreateWidget "/Game/l014519j/Widget/DSBP_Timer.DSBP_Timer_C"))
      (UserInterface|Viewport|AddtoViewport _returnvalue 0))
    (:then_1
      (bind _returnvalue_2 (UserInterface|CreateWidget "/Game/l014519j/Widget/W_Timer_Int.W_Timer_Int_C"))
      (UserInterface|Viewport|AddtoViewport _returnvalue_2 0))))

(fn ConstructionScript)