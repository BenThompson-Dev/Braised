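; Shrinking safe-zone sphere of light that closes in as darkness fills, opening the game-over map when full.
; A timeline drives fill amount, inverse actor scale and the UI darkness bar; light pickups reverse it to a target, then it resumes forward.
; Leaving the sphere starts looping player damage, post-process, camera fade and darkness music; re-entering clears them and restores health.
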(event OnComponentBeginOverlap(StaticMesh)
  (params (OverlappedComponent :type Primitive%20Component%20Object%20Reference) (OtherActor :type Actor%20Object%20Reference) (OtherComp :type Primitive%20Component%20Object%20Reference) (OtherBodyIndex :type Integer) (bFromSweep :type Boolean) (SweepResult :type Hit%20Result%20Structure%20%28by%20ref%29))
  ;[1 1 1] Stops Damage When in Sphere - l014519j
  (Class|BPIPlayer|IDarknessMusic(Message) OtherActor false)
  (if (Actor|ActorHasTag OtherActor "Player")
    (bind _playerref (Class|BPIPlayer|IGetPlayerRef(Message) OtherActor))
    (Default|ChangePostProcessEnabled _playerref false)
    (Utilities|Time|ClearandInvalidateTimerbyHandle (Variables|Default|GetHealthTimer))
    (CameraFades|StopCameraFade (Game|GetPlayerCameraManager 0))
    ;;[1 0 0] Update health back to 100 - l014519j
    (Class|BPIHealth|ISetHealth(Message) (Pawn|GetControlledPawn (Game|GetPlayerController 0)) 1e+02)))

(event OnComponentEndOverlap(StaticMesh)
  (params (OverlappedComponent :type Primitive%20Component%20Object%20Reference) (OtherActor :type Actor%20Object%20Reference) (OtherComp :type Primitive%20Component%20Object%20Reference) (OtherBodyIndex :type Integer))
  ;[1 1 1] Starts Darkness Damage on timer when outside sphere - l014519j
  (Class|BPIPlayer|IDarknessMusic(Message) OtherActor true)
  (if (Actor|ActorHasTag OtherActor "Player")
    (bind _playerref (Class|BPIPlayer|IGetPlayerRef(Message) OtherActor))
    (Default|ChangePostProcessEnabled _playerref true)
    (bind _returnvalue (Utilities|Time|SetTimerbyEvent (delegate Custom|DarknessDmgUpdate) 2.0 true 2.0))
    (Variables|Default|SetHealthTimer _returnvalue)
    (CameraFades|StartCameraFade :self (Game|GetPlayerCameraManager 0) :ToAlpha 1.0 :Duration 23.0)))

(event Custom|ReverseTimeline
  (bind _scalebounds (Variables|Default|GetscaleBounds))
  (bind (_x _y) (Math|Vector2D|BreakVector2D _scalebounds))
  ;[1 1 1 1 24] t014172k - Darkness sphere scaling
  ;;[1 0 0] Handles setting the timeline direction
  (Components|Timeline|SetPlayRate (Variables|Default|GetScaleTimeline) (Variables|Default|GetreverseRate))
  (bind (_direction _alpha) (Timeline|ScaleTimeline Reverse)
    (:Update
      ;;[1 0 0] Updates the sphere's scale
      (bind _output_get (Variables|Default|SetfillAmount _alpha))
      (Transformation|SetActorScale3D (Math|Conversions|ToVector(Float) (Math|Float|MapRangeClamped _output_get (Variables|Default|GetminValue) (Variables|Default|GetmaxValue) _y _x)))
      (CallFunction|UpdateDarknessBar)
      ;;[1 0 0] Checks if the timeline is running in reverse and the scale increase amount has been reached
      (if (Utilities|Enum|Equal(Enum) _direction "Backward")
        (if (<= (Variables|Default|GetfillAmount) (Variables|Default|GettargetAmount))
          (CallFunction|StartTimeline))))
    (:Finished
      ;;[0.1126 1 0.07286] Calls Darkness Death Function - l014519j
      (CallFunction|DarknessDeath))))

(event Custom|StartTimeline
  (bind _scalebounds (Variables|Default|GetscaleBounds))
  (bind (_x _y) (Math|Vector2D|BreakVector2D _scalebounds))
  ;[1 1 1 1 24] t014172k - Darkness sphere scaling
  ;;[1 0 0] Handles setting the timeline direction
  (Components|Timeline|SetPlayRate (Variables|Default|GetScaleTimeline) (Variables|Default|GetinitialRate))
  (bind (_direction _alpha) (Timeline|ScaleTimeline Play)
    (:Update
      ;;[1 0 0] Updates the sphere's scale
      (bind _output_get (Variables|Default|SetfillAmount _alpha))
      (Transformation|SetActorScale3D (Math|Conversions|ToVector(Float) (Math|Float|MapRangeClamped _output_get (Variables|Default|GetminValue) (Variables|Default|GetmaxValue) _y _x)))
      (CallFunction|UpdateDarknessBar)
      ;;[1 0 0] Checks if the timeline is running in reverse and the scale increase amount has been reached
      (if (Utilities|Enum|Equal(Enum) _direction "Backward")
        (if (<= (Variables|Default|GetfillAmount) (Variables|Default|GettargetAmount))
          (CallFunction|StartTimeline))))
    (:Finished
      ;;[0.1126 1 0.07286] Calls Darkness Death Function - l014519j
      (CallFunction|DarknessDeath))))

(event Custom|SetPercentage
  (params (fillAmount :type Float%20%28single-precision%29))
  (bind _scalebounds (Variables|Default|GetscaleBounds))
  (bind (_x _y) (Math|Vector2D|BreakVector2D _scalebounds))
  ;[1 1 1 1 24] t014172k - Darkness sphere scaling
  ;;[1 0 0] Handles setting the current position of the timeline based on percentage
  (bind (_direction _alpha) (Timeline|ScaleTimeline SetNewTime)
    (:Update
      ;;[1 0 0] Updates the sphere's scale
      (bind _output_get (Variables|Default|SetfillAmount _alpha))
      (Transformation|SetActorScale3D (Math|Conversions|ToVector(Float) (Math|Float|MapRangeClamped _output_get (Variables|Default|GetminValue) (Variables|Default|GetmaxValue) _y _x)))
      (CallFunction|UpdateDarknessBar)
      ;;[1 0 0] Checks if the timeline is running in reverse and the scale increase amount has been reached
      (if (Utilities|Enum|Equal(Enum) _direction "Backward")
        (if (<= (Variables|Default|GetfillAmount) (Variables|Default|GettargetAmount))
          (CallFunction|StartTimeline))))
    (:Finished
      ;;[0.1126 1 0.07286] Calls Darkness Death Function - l014519j
      (CallFunction|DarknessDeath))))

(event Custom|UpdateDarknessBar
  ;[1 1 1] t014172k - Updates the darkness bar percentage
  (Class|BPIUI|ISetDarknessBar(Message) (Variables|Default|GetdarknessBar) (Math|Float|MapRangeClamped (Variables|Default|GetfillAmount) (Variables|Default|GetminValue) (Variables|Default|GetmaxValue) 0.0 1.0)))

(event Custom|DarknessDmgUpdate
  ;[1 1 1] Starts Darkness Damage on timer when outside sphere - l014519j
  (Class|BPIDamage|TakeDamage(Message) (Game|GetPlayerCharacter 0) 1e+01))

(event Custom|Darkness%20Death
  ;[1 1 1] New Event called for death when the Darkness bar Fills - l014519j
  (if (>= (Variables|Default|GetfillAmount) (Variables|Default|GetmaxValue))
    (Game|OpenLevel(byName) "GameOverMap")))

(event EventIIncreaseLight
  (params (lightIncreaseAmount :type Integer))
  ;[1 1 1 1 24] t014172k - Darkness sphere scaling
  ;;[1 0 0] Reverses the timeline to increase the amount of light
  (Variables|Default|SettargetAmount (Math|Float|Clamp(Float) (- (Variables|Default|GetfillAmount) (Math|Conversions|ToFloat(Integer) lightIncreaseAmount)) (Variables|Default|GetminValue) (Variables|Default|GetmaxValue)))
  (CallFunction|ReverseTimeline))

(event EventIInit
  ;[1 1 1 1 24] t014172k - Darkness sphere scaling
  ;;[1 0 0] Gets the player UI widget
  (bind _ui (Class|BPIPlayer|IGetUI(Message) (Pawn|GetControlledPawn (Game|GetPlayerController 0))))
  (Variables|Default|SetdarknessBar _ui)
  (CallFunction|UpdateDarknessBar)
  ;;[1 0 0] Starts the shrinking timeline
  (CallFunction|SetPercentage (Variables|Default|GetfillAmount))
  (CallFunction|StartTimeline))

(fn ConstructionScript)

(fn IGetHealth)

(fn IGetGM
  (return 0))

(fn IGetJournalPages
  (return 0))

(fn IGetSec
  (return 0))

(fn IGetTimer
  (return 0))