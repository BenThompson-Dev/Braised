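; BP_DarknessSphereTest is a test sphere actor for a darkness mechanic, scaling its mesh via a timeline on BeginPlay.
; Leaving the sphere reverses the timeline, while entering clears the damage timer and stops the camera fade.
; The looping player-damage timer, camera fade-out and game-mode percent-based scaling are disconnected and never run, despite a comment saying exit starts damage.
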(event OnComponentBeginOverlap(StaticMesh)
  (params (OverlappedComponent :type Primitive%20Component%20Object%20Reference) (OtherActor :type Actor%20Object%20Reference) (OtherComp :type Primitive%20Component%20Object%20Reference) (OtherBodyIndex :type Integer) (bFromSweep :type Boolean) (SweepResult :type Hit%20Result%20Structure%20%28by%20ref%29))
  ;[1 1 1] Stops Damage When in Sphere - l014519j
  (Utilities|Time|ClearandInvalidateTimerbyHandle (Variables|Default|GetHealth))
  (CameraFades|StopCameraFade (Game|GetPlayerCameraManager 0)))

(event OnComponentEndOverlap(StaticMesh)
  (params (OverlappedComponent :type Primitive%20Component%20Object%20Reference) (OtherActor :type Actor%20Object%20Reference) (OtherComp :type Primitive%20Component%20Object%20Reference) (OtherBodyIndex :type Integer))
  ;[1 1 1] Starts Darkness Damage on timer when outside sphere - l014519j
  (bind _newtrack_1 (Timeline|Timeline_1 Reverse)
    (:Update
      (Transformation|SetWorldScale3D (Variables|Default|GetStaticMesh) (Math|Conversions|ToVector(Float) _newtrack_1)))))

(event Custom|Update
  ;[1 1 1] Starts Darkness Damage on timer when outside sphere - l014519j
  (Class|BPIDamage|TakeDamage(Message) (Game|GetPlayerCharacter 0) 1e+01))

(event EventTick
  (params (DeltaSeconds :type Float%20%28single-precision%29))
  ;[1 1 1] Scales Darkness Sphere - l014519j
)

(event EventBeginPlay
  (bind _newtrack_1 (Timeline|Timeline_1 Play)
    (:Update
      (Transformation|SetWorldScale3D (Variables|Default|GetStaticMesh) (Math|Conversions|ToVector(Float) _newtrack_1)))))

(fn ConstructionScript)