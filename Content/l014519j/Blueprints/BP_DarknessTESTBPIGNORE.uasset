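; Test darkness hazard actor that sends a damage message to any actor that begins overlapping it.
; A custom DarknessDamage event, not called within this graph, hits the player character four times at timed intervals when passed a true overlap flag.
; Leaving the Box stops the camera fade.
; Disconnected draft logic holds the fade-to-dark, an overlap check and a slow Box slide along X, so none of it runs.
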(event OnComponentEndOverlap(Box)
  (params (OverlappedComponent :type Primitive%20Component%20Object%20Reference) (OtherActor :type Actor%20Object%20Reference) (OtherComp :type Primitive%20Component%20Object%20Reference) (OtherBodyIndex :type Integer))
  (CameraFades|StopCameraFade (Game|GetPlayerCameraManager 0)))

(event Custom|Darkness%20Damage
  (params (Is%20Overlapped :type Boolean))
  (if Is%20Overlapped
    (Class|BPIDamage|TakeDamage(Message) (Game|GetPlayerCharacter 0) 25.0)
    (Utilities|FlowControl|Delay 2.5)
    (Class|BPIDamage|TakeDamage(Message) (Game|GetPlayerCharacter 0) 25.0)
    (Utilities|FlowControl|Delay 2.5)
    (Class|BPIDamage|TakeDamage(Message) (Game|GetPlayerCharacter 0) 25.0)
    (Utilities|FlowControl|Delay 2.5)
    (Class|BPIDamage|TakeDamage(Message) (Game|GetPlayerCharacter 0) 25.0)))

(event Collision|EventActorBeginOverlap
  (params (OtherActor :type Actor%20Object%20Reference))
  (Class|BPIDamage|TakeDamage(Message) OtherActor 1e+01))

(fn ConstructionScript)