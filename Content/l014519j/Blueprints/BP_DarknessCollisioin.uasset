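; Darkness zone actor whose sphere is a safe area, punishing the player for leaving it with damage and a darkening screen.
; Ending overlap with DarknessSphere starts a looping damage timer on the player and a slow camera and audio fade; actor overlap cancels both, with neither event filtering actors.
; Tick polls a percent value from the GameMode via interface, snapping the sphere to a small or large radius around a threshold.
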(event OnComponentEndOverlap(DarknessSphere)
  (params (OverlappedComponent :type Primitive%20Component%20Object%20Reference) (OtherActor :type Actor%20Object%20Reference) (OtherComp :type Primitive%20Component%20Object%20Reference) (OtherBodyIndex :type Integer))
  ;[1 1 1] Starts Darkness Damage on timer when outside sphere - l014519j
  (bind _returnvalue (Utilities|Time|SetTimerbyEvent (delegate Custom|Update) 2.0 true 2.0))
  (Variables|Default|SetHealth _returnvalue)
  (CameraFades|StartCameraFade :self (Game|GetPlayerCameraManager 0) :ToAlpha 1.0 :Duration 2e+01 :bShouldFadeAudio true :bHoldWhenFinished true))

(event Custom|Update
  ;[1 1 1] Starts Darkness Damage on timer when outside sphere - l014519j
  (Class|BPIDamage|TakeDamage(Message) (Game|GetPlayerCharacter 0) 1e+01))

(event Collision|EventActorBeginOverlap
  (params (OtherActor :type Actor%20Object%20Reference))
  ;[1 1 1] Stops Damage When in Sphere - l014519j
  (Utilities|Time|ClearandInvalidateTimerbyHandle (Variables|Default|GetHealth))
  (CameraFades|StopCameraFade (Game|GetPlayerCameraManager 0)))

(event EventTick
  (params (DeltaSeconds :type Float%20%28single-precision%29))
  ;[1 1 1] Shrinking the Darkness Sphere - l014519j
  (bind _percent (Class|BPIPercentage|IGetPercent(Message) (Game|GetGameMode)))
  (bind _output_get (Variables|Default|SetPercent _percent))
  (if (<= _output_get 1.8e+02)
    (Components|Sphere|SetSphereRadius (Variables|Default|GetDarkness%20Sphere) 5e+02 true)
    (Development|PrintString "Shrink")
    (else
      (Components|Sphere|SetSphereRadius (Variables|Default|GetDarkness%20Sphere) 2457.0 true)
      (Development|PrintString "Fail"))))

(fn ConstructionScript)