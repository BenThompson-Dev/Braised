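; BP_Pen is a creature pen that starts broken and is repaired with wood.
; Interface calls add wood to its inventory component and check the count against the requirement; once met, it broadcasts the repair and swaps to the repaired mesh.
; While repaired, its collider tells entering creatures they are penned and has the referenced spawner produce that creature's food, stopping when an actor leaves.
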(event OnComponentBeginOverlap(PenCollider)
  (params (OverlappedComponent :type Primitive%20Component%20Object%20Reference) (OtherActor :type Actor%20Object%20Reference) (OtherComp :type Primitive%20Component%20Object%20Reference) (OtherBodyIndex :type Integer) (bFromSweep :type Boolean) (SweepResult :type Hit%20Result%20Structure%20%28by%20ref%29))
  ;[1 1 1] b014818k - Creature enters / leaves pen
  (if (Variables|Default|GetisRepaired)
    (Class|BPIBaseCreature|IIsinPen(Message) OtherActor true)
    (bind (_creaturereference _creaturefoodtype _creaturefoodid _spawnedfoodprogress) (Class|BPIBaseCreature|IGetCreatureReference(Message) OtherActor true))
    (if (== _creaturereference OtherActor)
      (Class|BPIFood|ISpawnFood(Message) (Variables|Default|GetspawnerReference) _creaturefoodid _spawnedfoodprogress))))

(event OnComponentEndOverlap(PenCollider)
  (params (OverlappedComponent :type Primitive%20Component%20Object%20Reference) (OtherActor :type Actor%20Object%20Reference) (OtherComp :type Primitive%20Component%20Object%20Reference) (OtherBodyIndex :type Integer))
  ;[1 1 1] b014818k - Creature enters / leaves pen
  (if (Variables|Default|GetisRepaired)
    (Class|BPIBaseCreature|IGetCreatureReference(Message) OtherActor false)
    (Default|IStopSpawnFood (Variables|Default|GetspawnerReference))))

(event Custom|Init
  ;[1 1 1] t014172k - Broken pen is initialised
  (Variables|Default|SetcurrentWood 0)
  (Variables|Default|SetisRepaired false)
  (Variables|Default|SetisInUse false)
  (Default|IInit (Variables|Default|GetBPC_Inventory))
  (CallFunction|UpdateMesh))

(event Custom|PenFixed
  ;[1 1 1] t014172k - Handles tracking the pen as fixed
  (Variables|Default|SetisRepaired true)
  (Default|CallPenRepaired self (Variables|Default|GetpenIndex))
  (CallFunction|UpdateMesh))

(event EventIAddWood
  (params (item :type BP%20Pickup%20Item%20Wood%20Object%20Reference))
  ;[1 1 1] t014172k - Wood is added into the pen's inventory
  (bind _iteminfo (Class|BPIItem|IGetItem(Message) item))
  (Development|PrintString (.itemName (Utilities|Struct|BreakStruct_InventoryItem _iteminfo)))
  (Default|AddItem (Variables|Default|GetBPC_Inventory) _iteminfo))

(fn ConstructionScript)

(fn UpdateMesh
  ;[1 1 1] Updates the pen's mesh based on the inventory
  (if (Variables|Default|GetisRepaired)
    (bind _returnvalue (Components|StaticMesh|SetStaticMesh (Variables|Default|GetStaticMesh) "/Game/Assets/Forest/SM_Pen2.SM_Pen2"))
    (else
      (Components|StaticMesh|SetStaticMesh (Variables|Default|GetStaticMesh) "/Game/Assets/Forest/SM_PenBroken.SM_PenBroken"))))

(fn ICheckWood
  ;[1 1 1] Checks if the wood was succesfully added to the inventory
  (bind _item (Default|GetItem (Variables|Default|GetBPC_Inventory))) ; Only one item in inventory so 0th index\ncan always be passed in
  (Development|PrintString (.itemName (Utilities|Struct|BreakStruct_InventoryItem _item)))
  (if (>= (.itemCount (Utilities|Struct|BreakStruct_InventoryItem _item)) (Variables|Default|GetwoodRequired))
    (CallFunction|PenFixed))
  (return true))

(fn ICreatureinPenBoolOutput
  (return false))

(fn IEatFood
  (params (foodReference :type Actor%20Object%20Reference))
  (return false))

(fn IGetCreatureReference
  (params (inPen :type Boolean)))

(fn IGetFoodProgressGain
  (return 0.0))

(fn IGetFoodType
  (return "NewEnumerator0"))