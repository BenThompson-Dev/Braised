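; Fungus creature character, a child Blueprint that moves by repeated hops and upgrades through levels.
; A hop request fills a scaled distance array, then a looping timer launches the character along the raw direction with vertical force until the hop count is reached.
; The pen event sets that vertical force.
; Upgrades raise light gain, progress cap and spawned food progress, with early levels also swapping materials or mesh.
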(event Custom|Hop2
  ;[1 1 1] Launches the player in the hop direction.
  (if (== (stale EventIHop HopCount) (Variables|Default|GethopIndex))
    (Utilities|Time|ClearandInvalidateTimerbyHandle (Variables|Default|GetHopTimerHandle))
    (else
      (Character|LaunchCharacter (Math|Vector|MakeVector (.X (Math|Vector|BreakVector (stale EventIHop Direction))) (.Y (Math|Vector|BreakVector (stale EventIHop Direction))) (Variables|Default|GetverticalJumpForce)) false false)
      (Math|Integer|IncrementInt (Variables|Default|GethopIndex)))))

(event EventIHop
  (params (HopCount :type Integer) (Direction :type Vector :default "0, 0, 0"))
  ;[1 1 1] Gets the total hop distance and divides it by the hop count, then inverses the index and adds it to a new vector array.
  (Variables|Default|SethopIndex 0)
  (for _index (range 1 HopCount)
    (Utilities|Array|Add (Variables|Default|GethopDistances) (/ Direction (Math|Float|MapRangeClamped (Math|Conversions|ToFloat(Integer) _index) 1.0 (Math|Conversions|ToFloat(Integer) HopCount) (Math|Conversions|ToFloat(Integer) HopCount) 1.0))))
  (bind _returnvalue (Utilities|Time|SetTimerbyFunctionName 0 "Hop2" 1.4 true))
  (Variables|Default|SetHopTimerHandle _returnvalue))

(event EventIIsinPen
  (params (isInPen :type Boolean))
  (|CallParentFunction isInPen)
  (Variables|Default|SetverticalJumpForce 2e+02))

(fn ConstructionScript
  (|CallParentFunction))

(fn Upgrade
  (|CallParentFunction)
  (switch int (Variables|Default|GetcurrentLevel)
    (:1
      (Variables|Default|SetlightProgressGain 15.0)
      (Variables|Default|SetmaxProgress 125.0)
      (Variables|Default|SetcreatureSpawnedFoodProgress 5.0)
      (for _index (range 0 2)
        (Utilities|Array|SetArrayElem (Variables|Default|GetdefaultMaterials) _index "/Game/Assets/Creature/Mushroom_Upgrade1.Mushroom_Upgrade1")
        (Rendering|Material|SetMaterial (Variables|Character|GetMesh) _index "/Game/Assets/Creature/Mushroom_Upgrade1.Mushroom_Upgrade1")))
    (:2
      (Variables|Default|SetlightProgressGain 3e+01)
      (Variables|Default|SetmaxProgress 1.5e+02)
      (Variables|Default|SetcreatureSpawnedFoodProgress 1e+01)
      (Class|SkinnedMeshComponent|SetSkeletalMesh (Variables|Character|GetMesh) "/Engine/Tutorial/SubEditors/TutorialAssets/Character/TutorialTPP.TutorialTPP" true)
      (Rendering|Material|SetMaterial (Variables|Character|GetMesh) 0 "/Game/Assets/Textures/Materials/Mat_RuinsWood_Mat.Mat_RuinsWood_Mat"))
    (:3
      (Variables|Default|SetlightProgressGain 6e+01)
      (Variables|Default|SetmaxProgress 175.0)
      (Variables|Default|SetcreatureSpawnedFoodProgress 15.0))
    (:4
      (Variables|Default|SetlightProgressGain 9e+01)
      (Variables|Default|SetmaxProgress 2e+02)
      (Variables|Default|SetcreatureSpawnedFoodProgress 2e+01))))