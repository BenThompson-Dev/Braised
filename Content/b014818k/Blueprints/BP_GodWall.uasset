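; BP_GodWall is a progression gate that removes its blocking mesh once the player has released enough maxed creatures.
; On init it binds to every CH_BaseCreature's released-at-max event, tallying Fungus, Fruit and Cactus releases by class display name.
; Each type unlocks at two releases, and when all unlock flags are set, MeshBlock is destroyed.
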(event Custom|AddCount
  (params (Creature :type CH%20Base%20Creature%20Object%20Reference))
  (bind _unlockscount (Variables|Default|GetunlocksCount))
  (switch string (Utilities|GetClassDisplayName (Utilities|GetClass Creature))
    (:CH_Fungus_C
      (Utilities|Array|SetArrayElem _unlockscount 0 (+ (Utilities|Array|Get(acopy) _unlockscount) 1)))
    (:CH_Fruit_C
      (Utilities|Array|SetArrayElem (Variables|Default|GetunlocksCount) 1 (+ (Utilities|Array|Get(acopy) (Variables|Default|GetunlocksCount) 1) 1)))
    (:CH_Cactus_C
      (Utilities|Array|SetArrayElem (Variables|Default|GetunlocksCount) 2 (+ (Utilities|Array|Get(acopy) (Variables|Default|GetunlocksCount) 2) 1))))
  (for (_array_element _array_index) (Variables|Default|GetunlocksCount)
    (if (>= _array_element 2)
      (Utilities|Array|SetArrayElem (Variables|Default|GetunlocksBool) _array_index true)))
  (if (not (Utilities|Array|ContainsItem (Variables|Default|GetunlocksBool) false))
    (Actor|DestroyActor (Variables|Default|GetmeshBlock))))

(event Collision|EventActorBeginOverlap
  (params (OtherActor :type Actor%20Object%20Reference)))

(event EventIInit
  (bind _outactors (Actor|GetAllActorsOfClass "/Game/b014818k/Blueprints/BaseCreature/CH_BaseCreature.CH_BaseCreature_C"))
  (for _array_element _outactors
    (EventDispatchers|BindEventtoCreatureReleasedatMax _array_element (delegate Custom|AddCount))))

(fn ConstructionScript)