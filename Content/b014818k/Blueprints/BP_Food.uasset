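; BP_Food is a food actor that other actors can eat, linked to the spawner that created it.
; Overlapping its FoodCollider sends an eat-food interface message to the other actor, passing itself.
; The destroy-food interface event marks it picked up and notifies a valid spawner before destroying it, or prints a warning and still destroys it.
; The creature-related interface functions return only default values.
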(event OnComponentBeginOverlap(FoodCollider)
  (params (OverlappedComponent :type Primitive%20Component%20Object%20Reference) (OtherActor :type Actor%20Object%20Reference) (OtherComp :type Primitive%20Component%20Object%20Reference) (OtherBodyIndex :type Integer) (bFromSweep :type Boolean) (SweepResult :type Hit%20Result%20Structure%20%28by%20ref%29))
  (Class|BPIBaseCreature|IEatFood(Message) OtherActor self))

(event EventBeginPlay)

(event Collision|EventActorBeginOverlap
  (params (OtherActor :type Actor%20Object%20Reference)))

(event EventTick
  (params (DeltaSeconds :type Float%20%28single-precision%29)))

(event EventIDestroyFood
  (if (Utilities|IsValid (Variables|Default|GetspawnerReference))
    (Variables|Default|SetpickedUp true)
    (Default|IFoodPickedUp (Variables|Default|GetspawnerReference))
    (Actor|DestroyActor)
    (else
      (Development|PrintString "spawner isnt valid")
      (Actor|DestroyActor))))

(fn ConstructionScript)

(fn ICreatureinPenAI
  (return false))

(fn IGetCreatureReference
  (params (inPen :type Boolean))
  (return 0 "NewEnumerator0" 0.0))