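; BP_FoodSpawner spawns BP_Food pickups at its own location, passing them a food type, progress gain and spawner reference.
; World spawners spawn food on BeginPlay, while ISpawnFood starts a one-shot timer to spawn food if none is out.
; IFoodPickedUp clears the spawned flag and restarts that timer, passing zero gain so the stored type and gain are kept.
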(event Custom|SpawnTimer
  (bind _returnvalue (Game|SpawnActorfromClass "/Game/b014818k/Blueprints/BP_Food.BP_Food_C" (Transformation|GetActorTransform self) "Undefined" 0 0))
  (Variables|/Game/b014818k/Blueprints/BP_Food.BP_Food_C|SetfoodProgressGain _returnvalue (Variables|Default|GetfoodProgressGain))
  (Variables|/Game/b014818k/Blueprints/BP_Food.BP_Food_C|SetfoodType _returnvalue (Variables|Default|GetspawnerFoodType))
  (Variables|Default|SethasSpawnedFood true)
  ;[1 1 1] Replace later with dispatchers
  (Variables|/Game/b014818k/Blueprints/BP_Food.BP_Food_C|SetspawnerReference _returnvalue self))

(event EventBeginPlay
  (if (Variables|Default|GetisWorldFoodSpawner)
    (bind _returnvalue (Game|SpawnActorfromClass "/Game/b014818k/Blueprints/BP_Food.BP_Food_C" (Transformation|GetActorTransform self) "Undefined" 0 0))
    (Variables|/Game/b014818k/Blueprints/BP_Food.BP_Food_C|SetfoodProgressGain _returnvalue (Variables|Default|GetfoodProgressGain))
    (Variables|/Game/b014818k/Blueprints/BP_Food.BP_Food_C|SetfoodType _returnvalue (Variables|Default|GetspawnerFoodType))
    (Variables|Default|SethasSpawnedFood true)
    ;[1 1 1] Replace later with dispatchers
    (Variables|/Game/b014818k/Blueprints/BP_Food.BP_Food_C|SetspawnerReference _returnvalue self)))

(event EventISpawnFood
  (params (spawnerFoodType :type Enum_FoodTypes%20Enum :default "NewEnumerator0") (foodProgressGain :type Float%20%28single-precision%29))
  (if (!= foodProgressGain 0.0)
    (Variables|Default|SetspawnerFoodType spawnerFoodType)
    (Variables|Default|SetfoodProgressGain foodProgressGain))
  (if (not (Variables|Default|GethasSpawnedFood))
    (Utilities|Time|SetTimerbyEvent (delegate Custom|SpawnTimer) (Variables|Default|GetspawnFoodTimer))))

(event EventIFoodPickedUp
  (Variables|Default|SethasSpawnedFood false)
  (CallFunction|ISpawnFood "NewEnumerator0" 0.0))

(fn ConstructionScript)