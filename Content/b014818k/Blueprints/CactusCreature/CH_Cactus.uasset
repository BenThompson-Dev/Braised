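; CH_Cactus is the cactus creature, a child Blueprint that extends its parent's interaction and upgrade behavior.
; Interacting runs the parent logic, then sends a sub-page unlock message to the game mode with Enabled set to false.
; Upgrade calls the parent, then sets rising light progress gain, maximum progress and spawned food progress for each of four levels.
; Material and mesh changes per level are only placeholder print strings.
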(event EventBeginPlay)

(event Collision|EventActorBeginOverlap
  (params (OtherActor :type Actor%20Object%20Reference)))

(event EventIInteract
  (params (playerRef :type Character%20Object%20Reference) (Jakesplayerref :type CH%20Player%20Object%20Reference))
  (|CallParentFunction playerRef Jakesplayerref)
  (Class|BPIGM|IUnlockSubPages(Message) (Game|GetGameMode) "NewEnumerator2" false))

(event EventTick
  (params (DeltaSeconds :type Float%20%28single-precision%29)))

(fn ConstructionScript
  (|CallParentFunction))

(fn Upgrade
  (|CallParentFunction)
  (switch int (Variables|Default|GetcurrentLevel)
    (:1
      (Variables|Default|SetlightProgressGain 1e+01)
      (Variables|Default|SetmaxProgress 125.0)
      (Variables|Default|SetcreatureSpawnedFoodProgress 5.0)
      (Development|PrintString "Change Material"))
    (:2
      (Variables|Default|SetlightProgressGain 2e+01)
      (Variables|Default|SetmaxProgress 1.5e+02)
      (Variables|Default|SetcreatureSpawnedFoodProgress 1e+01)
      (Development|PrintString "Change Material"))
    (:3
      (Variables|Default|SetlightProgressGain 3e+01)
      (Variables|Default|SetmaxProgress 175.0)
      (Variables|Default|SetcreatureSpawnedFoodProgress 15.0)
      (Development|PrintString "Change Mesh"))
    (:4
      (Variables|Default|SetlightProgressGain 4e+01)
      (Variables|Default|SetmaxProgress 2e+02)
      (Variables|Default|SetcreatureSpawnedFoodProgress 2e+01)
      (Development|PrintString "Change Material"))))