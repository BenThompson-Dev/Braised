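; BP_PosterSign is an interactable poster sign that comes in four variants: Leabry, Draguy, Fungoo and God.
; On BeginPlay, its SignType selects the poster material applied to slot 1 of the static mesh.
; It always allows interaction, and interacting messages the GameMode through an interface to unlock the sub-page that matches the sign type.
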(event EventIInteract
  (params (playerRef :type Character%20Object%20Reference) (Jakesplayerref :type CH%20Player%20Object%20Reference))
  (bind _returnvalue (Game|GetGameMode))
  (bind _returnvalue_2 (Game|GetGameMode))
  (switch Utilities|FlowControl|Switch|SwitchonEnum_Signs (Variables|Default|GetSignType)
    (:NewEnumerator0
      (Class|BPIGM|IUnlockSubPages(Message) _returnvalue_2 "NewEnumerator1" true))
    (:NewEnumerator1
      (Class|BPIGM|IUnlockSubPages(Message) _returnvalue_2 "NewEnumerator2" true))
    (:NewEnumerator2
      (Class|BPIGM|IUnlockSubPages(Message) _returnvalue "NewEnumerator3" true))
    (:NewEnumerator3
      (Class|BPIGM|IUnlockSubPages(Message) _returnvalue "NewEnumerator4" true))))

(event EventBeginPlay
  (bind _staticmesh (Variables|Default|GetStaticMesh))
  (bind _staticmesh_2 (Variables|Default|GetStaticMesh))
  (switch Utilities|FlowControl|Switch|SwitchonEnum_Signs (Variables|Default|GetSignType)
    (:NewEnumerator0
      (Rendering|Material|SetMaterial _staticmesh_2 1 "/Game/Assets/Textures/Materials/leabry_Mat.leabry_Mat"))
    (:NewEnumerator1
      (Rendering|Material|SetMaterial _staticmesh_2 1 "/Game/Assets/Textures/Materials/draguy_poster_Mat.draguy_poster_Mat"))
    (:NewEnumerator2
      (Rendering|Material|SetMaterial _staticmesh 1 "/Game/Assets/Textures/Materials/Fungoo_Mat.Fungoo_Mat"))
    (:NewEnumerator3
      (Rendering|Material|SetMaterial _staticmesh 1 "/Game/Assets/Textures/Materials/god_poster_Mat.god_poster_Mat"))))

(fn ConstructionScript)

(fn ICanInteract
  (return true))