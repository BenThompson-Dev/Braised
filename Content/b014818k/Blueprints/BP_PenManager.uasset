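; BP_PenManager tracks creature pens and drives a map UI for teleporting a creature to a repaired pen.
; On init it binds each BP_Pen's repair event and creates UI_Map, then tries to disable every pen button, a step noted as not working.
; Repairs register pens by index and enable their buttons.
; Interacting with a creature opens the map; pressing a registered pen's button teleports that creature to the pen's location.
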(event Custom|PenRepaired
  (params (pen :type BP%20Pen%20Object%20Reference) (index :type Enum_Pens%20Enum :default "NewEnumerator0"))
  (bind _buttons (Variables|Default|Getbuttons))
  (bind (_value _returnvalue) (Utilities|Map|Find _buttons index))
  ;[1 1 1] t014172k - Called when a pen has been repaired
  (Utilities|Map|Add (Variables|Default|GetactivePens) index pen)
  (Development|PrintString "pen fixed")
  (if _returnvalue
    (Default|ChangePenAvailable (Variables|Default|GetmapWidget) true _value)
    (else
      (Development|PrintString "button not found"))))

(event EventISetCreatureRef
  (params (creatureRef :type Actor%20Object%20Reference))
  ;[1 1 1] Event after player interacts with creature (With reference to creatureRef)
  (bind _output_get (Variables|Default|SetcreatureRef creatureRef))
  ;[1 1 1] Opens Map Widget
  (Class|BPIPlayer|IShowTeleportMap(Message) (Variables|Default|GetmapWidget) _output_get))

(event EventIInit
  ;[1 1 1] t014172k - Initialises each of the pens
  (bind _outactors (Actor|GetAllActorsOfClass "/Game/b014818k/Blueprints/BP_Pen.BP_Pen_C"))
  (bind _output_get (Variables|Default|Setpens _outactors))
  (for _array_element _output_get
    (Default|Init _array_element)
    (EventDispatchers|BindEventtoPenRepaired _array_element (EventDispatchers|CreateEvent :!event Custom|PenRepaired)))
  ;[1 1 1] Sets up the pen buttons
  (bind _returnvalue (UserInterface|CreateWidget "/Game/b014818k/UI/UI_Map.UI_Map_C"))
  (bind _output_get_2 (Variables|Default|SetmapWidget _returnvalue))
  (Default|Init _output_get_2 self)
  (Class|BPIPlayer|ISetTeleportMapUI(Message) (Game|Player|GetPlayerPawn 0) (Variables|Default|GetmapWidget))
  (UserInterface|Viewport|AddtoViewport (Variables|Default|GetmapWidget) 0)
  ;[1 0 0] DOES NOT WORK - Disables the buttons when the game starts
  (bind _buttons (Default|GetButtons _output_get_2))
  (bind _output_get_3 (Variables|Default|Setbuttons _buttons))
  (bind _values (Utilities|Map|Values _output_get_3))
  (for _array_element_2 _values
    (Default|ChangePenAvailable (Variables|Default|GetmapWidget) false _array_element_2)))

(event EventIMapPenPressed
  (params (penIndex :type Enum_Pens%20Enum :default "NewEnumerator0"))
  (bind _activepens (Variables|Default|GetactivePens))
  (bind (_value _returnvalue) (Utilities|Map|Find _activepens penIndex))
  ;[1 1 1] t014172k - Called when a button on the map has been pressed
  (if _returnvalue
    (Development|PrintString "teleport creature")
    (Class|BPIBaseCreature|ITeleportCreature(Message) (Variables|Default|GetcreatureRef) (Transformation|GetActorLocation _value))
    (else
      (Development|PrintString "pen not found"))))

(fn ConstructionScript)

(fn ICheckWood
  (return false))