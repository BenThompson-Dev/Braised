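; Behavior tree task for creature AI that picks a random navigable destination around the controlled pawn.
; It samples a point within TargetRadius, writes it to the BBTarget blackboard key, and writes the unnormalized offset from the pawn to BBVelocity.
; The task succeeds when a point is found and fails otherwise.
; Creature pen and food interface functions are present only as default stubs.
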(event EventReceiveTickAI
  (params (OwnerController :type AI%20Controller%20Object%20Reference) (ControlledPawn :type Pawn%20Object%20Reference) (DeltaSeconds :type Float%20%28single-precision%29))
  (bind _returnvalue (Transformation|GetActorLocation ControlledPawn))
  (bind (_randomlocation _returnvalue_2) (Class|NavigationSystemV1|GetRandomLocationinNavigableRadius _returnvalue (Variables|Default|GettargetRadius) 0 0))
  (if _returnvalue_2
    (AI|BehaviorTree|SetBlackboardValueasVector (Variables|Default|GetBB_target) _randomlocation)
    (AI|BehaviorTree|SetBlackboardValueasVector (Variables|Default|GetBB_velocity) (- _randomlocation _returnvalue))
    (AI|BehaviorTree|FinishExecute true)
    (else
      (AI|BehaviorTree|FinishExecute false))))

(fn ICreatureinPenBoolOutput)

(fn IEatFood
  (params (foodReference :type Actor%20Object%20Reference))
  (return false))

(fn IGetCreatureReference
  (params (inPen :type Boolean))
  (return 0 "NewEnumerator0" 0 0.0))