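; Behavior tree task for base creatures that picks a random navigable point around the pawn as a wander target.
; Each AI tick it queries the pawn's pen interface; on a false result it sets the inside-pen blackboard key true, stores the point and finishes successfully.
; On a true result the task does not finish and keeps ticking.
; Its own interface functions are stubs, and a debug print chain is unconnected.
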(event EventReceiveTickAI
  (params (OwnerController :type AI%20Controller%20Object%20Reference) (ControlledPawn :type Pawn%20Object%20Reference) (DeltaSeconds :type Float%20%28single-precision%29))
  (bind _isinpen (Class|BPIBaseCreature|ICreatureinPenBoolOutput(Message) ControlledPawn))
  (if (not _isinpen)
    (Class|BTFunctionLibrary|SetBlackboardValueasBool (Variables|Default|GetBB_insidePen) true)
    (bind _randomlocation (Class|NavigationSystemV1|GetRandomLocationinNavigableRadius (Transformation|GetActorLocation ControlledPawn) (Variables|Default|GettargetRadius) 0 0))
    (if true
      (AI|BehaviorTree|SetBlackboardValueasVector (Variables|Default|GetBB_randomTarget) _randomlocation)
      (AI|BehaviorTree|FinishExecute true)
      (else
        (AI|BehaviorTree|FinishExecute true)))))

(fn ICreatureinPenBoolOutput)

(fn IGetCreatureReference
  (params (inPen :type Boolean))
  (return 0 "NewEnumerator0" 0.0))