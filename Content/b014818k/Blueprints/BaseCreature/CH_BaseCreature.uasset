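; Base creature character that players send to pens, feed to level up, and release to add light progress through the GameMode.
; Interacting opens the teleport map, or the release flow if penned; teleporting plays Niagara sparks and a timeline-driven material dissolve around the move.
; Matching food fills a proximity-shown progress bar while penned, triggering upgrades up to a max level.
; Interface messages link it to player, pen, food and UI.
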(event OnComponentBeginOverlap(ProgressBarCol)
  (params (OverlappedComponent :type Primitive%20Component%20Object%20Reference) (OtherActor :type Actor%20Object%20Reference) (OtherComp :type Primitive%20Component%20Object%20Reference) (OtherBodyIndex :type Integer) (bFromSweep :type Boolean) (SweepResult :type Hit%20Result%20Structure%20%28by%20ref%29))
  ;[1 1 1] Progress Bar visibility
  (if (== OtherActor (Game|Player|GetPlayerPawn 0))
    (Widget|SetVisibility (UserInterface|GetUserWidgetObject (Variables|Default|GetProgressBarWidget)) "Visible")))

(event OnComponentEndOverlap(ProgressBarCol)
  (params (OverlappedComponent :type Primitive%20Component%20Object%20Reference) (OtherActor :type Actor%20Object%20Reference) (OtherComp :type Primitive%20Component%20Object%20Reference) (OtherBodyIndex :type Integer))
  (bind _progressbarwidget (Variables|Default|GetProgressBarWidget))
  (bind _returnvalue (UserInterface|GetUserWidgetObject _progressbarwidget))
  ;[1 1 1] Progress Bar visibility
  (if (== OtherActor (Game|Player|GetPlayerPawn 0))
    (Utilities|IsValid _returnvalue
      (:Is%20Valid
        (Widget|SetVisibility _returnvalue "Hidden")))))

(event OnComponentActivated(ParticleDust)
  (params (Component :type Actor%20Component%20Object%20Reference) (bReset :type Boolean))
  ;[1 1 1] Enables / Disables the dust particle
)

(event Custom|ReleaseCreature
  (Class|BPIGM|IIncreaseLight(Message) (Game|GetGameMode) (Math|Float|Truncate (Variables|Default|GetlightProgressGain)))
  (Default|CreatureReleased (Variables|Default|GetPen%20Reference))
  (if (== (Variables|Default|GetcurrentLevel) (Variables|Default|GetmaxLevel))
    (Default|CallCreatureReleasedatMax self))
  (Actor|DestroyActor)
  (Default|PopUpUI :self (Variables|Default|Getjakesplayer) :enum "NewEnumerator3"))

(event EventIReleaseCreatureFinal
  ;[1 1 1] Releases the creature
  (CallFunction|ReleaseCreature))

(event EventITeleportCreature
  (params (PenLocation :type Vector :default "0, 0, 0"))
  (bind (_x _y _z) (Math|Vector|BreakVector PenLocation))
  (bind _niagarateleport (Variables|Default|GetNiagaraTeleport))
  ;[1 1 1] Teleport creature and update material
  (Effects|Components|ParticleSystem|SetColorParameter _niagarateleport "SparkBurstColor" "(R=0.258636,G=0.633258,B=0.875000,A=1.000000)")
  (Components|Activation|Activate _niagarateleport true)
  (Pawn|Components|CharacterMovement|DisableMovement (Variables|Character|GetCharacterMovement))
  (bind _returnvalue (Rendering|Material|CreateDynamicMaterialInstance (Variables|Character|GetMesh) 0 (Variables|Default|GetdissolveMaterialReference) "None" :!class /Script/Engine.PrimitiveComponent))
  (Variables|Default|SetdynamicMaterialReference _returnvalue)
  (bind _dissolvefloat (Timeline|DissolveMesh PlayFromStart)
    (:Update
      (Rendering|Material|SetScalarParameterValue (Variables|Default|GetdynamicMaterialReference) "Dissolve" _dissolvefloat :!class /Script/Engine.MaterialInstanceDynamic))
    (:Finished
      (Transformation|SetActorLocation (Math|Vector|MakeVector _x _y (+ _z 1e+02)) false false)
      (bind _dissolvefloat_2 (Timeline|ReverseDissolveMesh ReverseFromEnd)
        (:Update
          (Rendering|Material|SetScalarParameterValue (Variables|Default|GetdynamicMaterialReference) "Dissolve" _dissolvefloat_2 :!class /Script/Engine.MaterialInstanceDynamic))
        (:Finished
          (Pawn|Components|CharacterMovement|SetMovementMode (Variables|Character|GetCharacterMovement) "MOVE_Walking" 0)
          (Components|Activation|Deactivate (Variables|Default|GetNiagaraTeleport))
          (for (_array_element _array_index) (Variables|Default|GetdefaultMaterials)
            (Rendering|Material|SetMaterial (Variables|Character|GetMesh) _array_index _array_element)
            (Default|PopUpUI :self (Variables|Default|Getjakesplayer) :enum "NewEnumerator1")))))))

(event EventIInteract
  (params (playerRef :type Character%20Object%20Reference) (Jakesplayerref :type CH%20Player%20Object%20Reference))
  ;[1 1 1] t014172k - Interact function shows the teleport UI
  (Variables|Default|Setjakesplayer Jakesplayerref)
  (if (Variables|Default|GetinPen)
    (Class|BPIPlayer|IReleaseCreature(Message) playerRef)
    (else
      (Class|BPIPlayer|ISetCanMove(Message) playerRef false)
      (Class|BPIPlayer|IShowTeleportMap(Message) playerRef self))))

(event EventBeginPlay
  (Variables|Default|SetdefaultMaterials (Rendering|Material|GetMaterials (Variables|Character|GetMesh))))

(event EventIGetPen
  (params (Pen :type BP%20Pen%20Object%20Reference))
  (Variables|Default|SetPen%20Reference Pen))

(event EventIIsinPen
  (params (isInPen :type Boolean))
  (Variables|Default|SetinPen isInPen))

(event EventIPlayDustParticle
  (params (Play :type Boolean))
  ;[1 1 1] Enables / Disables the dust particle
  (if true
    (Components|Activation|Activate (Variables|Default|GetParticleDust) false)
    (else
      (Components|Activation|Deactivate (Variables|Default|GetParticleDust)))))

(fn ConstructionScript)

(fn Upgrade
  (bind _jakesplayer (Variables|Default|Getjakesplayer))
  (if (< (Variables|Default|GetcurrentLevel) (Variables|Default|GetmaxLevel))
    (Class|BPIGM|IIncreaseLight(Message) (Game|GetGameMode) (Math|Float|Truncate (Variables|Default|GetupgradeLightProgressGain)))
    (bind _result (Math|Integer|IncrementInt (Variables|Default|GetcurrentLevel))
      (:%20%20
        (Default|PopUpUI :self _jakesplayer :enum "NewEnumerator2" :Creature%20level _result)
        (bind _output_get (Variables|Default|SetcurrentProgress 0.0))
        (Class|BPIBaseCreature|IUpdateProgressBar(Message) (Variables|Default|GetProgressBarWidget) _output_get (Variables|Default|GetmaxProgress))
        (Components|Activation|Activate (Variables|Default|GetNiagaraEvolve) false)))
    (else
      (Default|PopUpUI :self _jakesplayer :enum "NewEnumerator4"))))

(fn LoadFoodType)

(fn IDontGetIt
  (params (NewParam1 :type CH%20Player%20Object%20Reference)))

(fn ICanInteract
  (return true))

(fn ICreatureinPenBoolOutput
  (return (Variables|Default|GetinPen)))

(fn IEatFood
  (params (foodReference :type Actor%20Object%20Reference))
  ;[1 1 1] Eats collided food if possible, calls upgrade if current progress reached max, updates progress bar ui.
  (bind _foodtype (Class|BPIFood|IGetFoodType(Message) foodReference))
  (if (and (Utilities|Enum|Equal(Enum) _foodtype (Variables|Default|GetcreatureFoodType)) (Variables|Default|GetinPen))
    (bind _foodprogressgain (Class|BPIFood|IGetFoodProgressGain(Message) foodReference))
    (Variables|Default|SetcurrentProgress (+ _foodprogressgain (Variables|Default|GetcurrentProgress)))
    (if (>= (Variables|Default|GetcurrentProgress) (Variables|Default|GetmaxProgress))
      (CallFunction|Upgrade))
    (Class|BPIBaseCreature|IUpdateProgressBar(Message) (UserInterface|GetUserWidgetObject (Variables|Default|GetProgressBarWidget)) (Variables|Default|GetcurrentProgress) (Variables|Default|GetmaxProgress))
    (Class|BPIBaseCreature|IDestroyFood(Message) foodReference)
    (return true)
    (else
      (Development|PrintString "Can't eat"))))

(fn IGetCreatureReference
  (params (inPen :type Boolean))
  (return true self (Variables|Default|GetcreatureFoodType) (Variables|Default|GetcreatureFoodItemID) (Variables|Default|GetcreatureSpawnedFoodProgress)))