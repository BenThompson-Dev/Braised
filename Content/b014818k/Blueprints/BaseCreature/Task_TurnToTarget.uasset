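; Behavior Tree task for base creature AI that turns the controlled pawn to face the Target location from the Blackboard.
; Each tick it builds a goal rotation from the look-at yaw and roll, keeping the pawn's current pitch.
; It eases the actor toward that rotation with RInterpTo at TurnSpeed and finishes successfully once within a small tolerance.
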(event EventReceiveTickAI
  (params (OwnerController :type AI%20Controller%20Object%20Reference) (ControlledPawn :type Pawn%20Object%20Reference) (DeltaSeconds :type Float%20%28single-precision%29))
  (bind _returnvalue (Transformation|GetActorLocation ControlledPawn))
  (bind _returnvalue_2 (Transformation|GetActorRotation ControlledPawn))
  (bind _target (Variables|Default|Gettarget))
  (bind _returnvalue_3 (Class|BTFunctionLibrary|GetBlackboardValueasVector _target))
  (bind _pitch (Math|Rotator|BreakRotator _returnvalue_2))
  (bind _returnvalue_4 (Math|Rotator|FindLookatRotation _returnvalue _returnvalue_3))
  (bind (_roll _pitch_2 _yaw) (Math|Rotator|BreakRotator _returnvalue_4))
  (bind _returnvalue_5 (Math|Rotator|MakeRotator _roll _pitch _yaw))
  ;[1 1 1] Check if the required rotation is met
  (if (Math|Rotator|Equal(Rotator) _returnvalue_2 _returnvalue_5 1.0)
    ;[1 1 1] Rotate the actor until the desired rotation is met
    (AI|BehaviorTree|FinishExecute true)
    (else
      (Transformation|SetActorRotation ControlledPawn (Math|Interpolation|RInterpTo _returnvalue_2 _returnvalue_5 (Utilities|Time|GetWorldDeltaSeconds) (Variables|Default|GetturnSpeed))))))