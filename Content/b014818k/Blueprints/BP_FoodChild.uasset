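; BP_FoodChild is a usable food item that can be fed to a hit actor and reports its food type and progress gain through interface getters.
; Using it sends an eat-food message to the hit actor, passing itself.
; On a destroy-food message it marks itself picked up and notifies its spawner if valid, then destroys itself either way.
; The creature-related interface functions return only stub values.
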(event EventBeginPlay
  (|CallParentFunction) ; This node is disabled and will not be called.\nDrag off pins to build functionality.
)

(event Collision|EventActorBeginOverlap
  (params (OtherActor :type Actor%20Object%20Reference)))

(event EventTick
  (params (DeltaSeconds :type Float%20%28single-precision%29)))

(event EventIDestroyFood
  (if (Utilities|IsValid (Variables|Default|GetspawnerReference))
    (Variables|Default|SetpickedUp true)
    (Class|BPIFood|IFoodPickedUp(Message) (Variables|Default|GetspawnerReference))
    (Actor|DestroyActor)
    (else
      (Development|PrintString "spawner isnt valid")
      (Actor|DestroyActor))))

(fn ConstructionScript
  (|CallParentFunction))

(fn UseFunctionality
  (params (hitActor :type Actor%20Object%20Reference))
  (Class|BPIBaseCreature|IEatFood(Message) hitActor self))

(fn ICreatureinPenBoolOutput
  (return false))

(fn IGetCreatureReference
  (params (inPen :type Boolean))
  (return 0 "NewEnumerator0" 0.0))

(fn IGetFoodProgressGain
  (return (Variables|Default|GetfoodProgressGain)))

(fn IGetFoodType
  (return (Variables|Default|GetfoodType)))