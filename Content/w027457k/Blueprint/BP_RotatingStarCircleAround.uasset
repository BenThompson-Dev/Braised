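; Actor that circles a target actor on a flat horizontal orbit, apparently a rotating star.
; Tick accumulates an angle from rotation speed, signed by the clockwise flag, and passes it to RotateActorAroundPoint.
; That function rotates a radius vector around Z by this angle plus a starting angle, then sets only location around the target's offset position.
; Without a valid target it does not move, so the stored initial location has no effect.
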(event EventBeginPlay
  ;[1 1 1] Sets initial location
  (Variables|Default|SetinitialLocation (Transformation|GetActorLocation)))

(event EventTick
  (params (DeltaSeconds :type Float%20%28single-precision%29))
  ;[1 1 1] Rotates on Tick
  (Variables|Default|SetcurrentRotation (+ (Variables|Default|GetcurrentRotation) (* (* (Variables|Default|GetrotationSpeed) DeltaSeconds) (Math|Float|SelectFloat 1.0 -1.0 (Variables|Default|Getclockwise)))))
  ;[1 1 1] Function Call
  (CallFunction|RotateActorAroundPoint self (Variables|Default|GettargetActor) (Variables|Default|GetinitialLocation) (Variables|Default|Getradius) (Variables|Default|GetstartingAngle) (Variables|Default|GetcurrentRotation)))

(fn ConstructionScript)

(fn RotateActorAroundPoint
  (params (Actor%20to%20Rotate :type Actor%20Object%20Reference) (Target%20Actor :type Actor%20Object%20Reference) (Target%20Location :type Vector) (Radius :type Float%20%28single-precision%29) (Angle :type Float%20%28single-precision%29) (Rotation%20Rate :type Float%20%28single-precision%29))
  ;[1 1 1] Set first variables
  (LocalVariables|Setactor_to_Rotate Actor%20to%20Rotate)
  (LocalVariables|Settarget_Actor Target%20Actor)
  (LocalVariables|Settarget_Location Target%20Location)
  (LocalVariables|Setlocal_Radius Radius)
  (LocalVariables|Setlocal_Angle Angle)
  (LocalVariables|Setrotation_Rate Rotation%20Rate)
  ;[1 1 1] Set location of object to the target actor
  (Utilities|IsValid (LocalVariables|Gettarget_Actor)
    (:Is%20Valid
      (LocalVariables|Settarget_Location (+ (Transformation|GetActorLocation (LocalVariables|Gettarget_Actor)) (Variables|Default|GetlocationOffset)))
      ;[1 1 1] Changes the location based on calculated rotation
      (Transformation|SetActorLocation Actor%20to%20Rotate (+ (LocalVariables|Gettarget_Location) (Math|Vector|RotateVectorAroundAxis (Math|Vector|MakeVector (LocalVariables|Getlocal_Radius) 0.0 0.0) (+ (LocalVariables|Getrotation_Rate) (LocalVariables|Getlocal_Angle)) "0, 0,1.000000")) false false)
      (return (LocalVariables|Gettarget_Location)))))