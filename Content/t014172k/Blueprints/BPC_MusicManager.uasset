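; Music manager component that plays a selectable background track through a spawned AmbientSound actor.
; Init spawns the actor at the world origin, sets an initial enum track and starts playback.
; SetSound stores the current track and looks up its sound in the MusicList map, falling back to S_ForestMusic when no entry exists.
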(event Custom|Init
  (CallFunction|SoundSetup)
  (CallFunction|SetSound "NewEnumerator0")
  (Audio|Components|Audio|Play (Variables|/Script/Engine.AmbientSound|GetAudioComponent (Variables|Default|GetambientSoundActor)) 0.0))

(event Custom|SoundSetup
  ;[1 1 1] Creates the ambient sound actor
  (bind _returnvalue (Game|SpawnActorfromClass "/Script/Engine.AmbientSound" (Math|Transform|MakeTransform "0, 0, 0") "Undefined" 0 0))
  (Variables|Default|SetambientSoundActor _returnvalue))

(event Custom|SetSound
  (params (newTrack :type Enum_Music%20Enum :default "NewEnumerator0"))
  ;[1 1 1] t014172k - Sets the new track
  (bind _output_get (Variables|Default|SetcurrentTrack newTrack))
  (if (.ReturnValue (Utilities|Map|Find (Variables|Default|GetmusicList) _output_get))
    (Audio|Components|Audio|SetSound (Variables|/Script/Engine.AmbientSound|GetAudioComponent (Variables|Default|GetambientSoundActor)) (.Value (Utilities|Map|Find (Variables|Default|GetmusicList) _output_get)))
    (else
      (Audio|Components|Audio|SetSound (Variables|/Script/Engine.AmbientSound|GetAudioComponent (Variables|Default|GetambientSoundActor)) "/Game/W015955i_WillW/Audio/Ambient/S_ForestMusic.S_ForestMusic"))))