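; Inventory component that stores items in a fixed number of slots, treating ItemID 0 as empty, and tracks the held item.
; Adds and replacements merge into non-full stacks through ItemCountChange, which clamps counts, writes overflow at the occupied-slot count index and clears emptied slots.
; Helpers compact slots, merge stacks, cycle the held index and total star items.
; Interface messages tell the owner to destroy pickups and update the held item.
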(event EventIInit
  ;[1 1 1] Sets the inventory to the correct length
  (while (< (Utilities|Array|Length (Variables|Default|Getinventory)) (Variables|Default|GetinventorySlots))
    (Utilities|Array|Add (Variables|Default|Getinventory) (Utilities|Struct|MakeStruct_InventoryItem "Item" 0 0 20 1e+01 0 0))))

(fn FindIteminInventory
  (params (newItem :type Struct%20Inventory%20Item%20Structure))
  ;[1 1 1] Checks to see if a (non-full) stack is in the inventory
  (bind (_array_element _array_index) (Utilities|Array|ForEachLoopwithBreak (Variables|Default|Getinventory) :!label _label) ; Loops through each inventory item
    (:LoopBody
      (LocalVariables|Setfound_Index _array_index) ; Stores the current index to use as the return value
      (bind _output_get (LocalVariables|Setis_Found (and (== (.itemID (Utilities|Struct|BreakStruct_InventoryItem newItem)) (.itemID (Utilities|Struct|BreakStruct_InventoryItem _array_element))) (!= (.itemCount (Utilities|Struct|BreakStruct_InventoryItem _array_element)) (.maxStack (Utilities|Struct|BreakStruct_InventoryItem _array_element))))))
      (if _output_get ; If item is found, breaks\nout of for loop
        (goto _label Break)))
    (:Completed
      (return (LocalVariables|Getfound_Index) (LocalVariables|Getis_Found)))))

(fn AddItem
  (params (newItem :type Struct%20Inventory%20Item%20Structure) (itemActorRef :type Actor%20Object%20Reference))
  (Utilities|FlowControl|Sequence
    (:then_0
      (bind (_index _found) (CallFunction|FindIteminInventory newItem)) ; Searches inventory for the item
      (if _found ; If item has been found
        (CallFunction|ItemCountChange _index newItem true) ; Adds the item count onto the existing item slot
        (else
          ;[1 1 1] Loops through the array to find the first empty space
          (bind (_array_element _array_index) (Utilities|Array|ForEachLoopwithBreak (Variables|Default|Getinventory) :!label _label)
            (:LoopBody
              (if (== (.itemID (Utilities|Struct|BreakStruct_InventoryItem _array_element)) 0)
                (Utilities|Array|SetArrayElem (Variables|Default|Getinventory) _array_index newItem) ; Sets the empty space to new item
                (Class|BPIPlayer|ICallDestroyItem(Message) (Components|GetOwner)) ; Calls event dispatcher to\ndestroy item
                (goto _label Break)))))))
    (:then_1
      (CallFunction|UpdateHeldItem))))

(fn ItemCountChange
  (params (itemIndexToChange :type Integer) (newItem :type Struct%20Inventory%20Item%20Structure) (isIncreasing :type Boolean))
  (bind _inventory (Variables|Default|Getinventory))
  (bind _output (Utilities|Array|Get(acopy) _inventory itemIndexToChange))
  (bind (_itemname _itemid _itemcount _maxstack) (Utilities|Struct|BreakStruct_InventoryItem _output))
  (bind (_itemname_2 _itemid_2 _itemcount_2 _maxstack_2 _feedingprogressgain _uiimage _itemactorref _foodtype _staticmesh _meshmaterial _newmeshmaterial) (Utilities|Struct|BreakStruct_InventoryItem _output))
  ;[1 1 1] Calculates change amount
  (LocalVariables|Setchange_Amount (.itemCount (Utilities|Struct|BreakStruct_InventoryItem newItem))) ; Sets the amount to change the\ncount by
  (if isIncreasing ; Checks to see if it is increasing or decreasing the count,\nand inverts the value if needed
    _
    (else
      (LocalVariables|Setchange_Amount (* (LocalVariables|Getchange_Amount) -1))))
  (LocalVariables|SetnewCount (+ (LocalVariables|Getchange_Amount) _itemcount))
  ;[1 1 1] Checks to see whether the object on the ground needs to be destroyed
  (if (<= (+ (LocalVariables|Getchange_Amount) _itemcount) 0) ; Checks to see if all of the objects can't be\npicked up
    (if (> (+ (LocalVariables|Getchange_Amount) _itemcount) _maxstack)
      _
      (else
        (Class|BPIPlayer|ICallDestroyItem(Message) (Components|GetOwner) :!label _label)))
    (else
      (goto _label)))
  ;[1 1 1] Creates new inventory struct item and adds it to the array
  (if (> (Math|Integer|Clamp(Integer) (+ (LocalVariables|Getchange_Amount) _itemcount) 0 _maxstack) 0)
    (Utilities|Array|SetArrayElem (Variables|Default|Getinventory) itemIndexToChange (Utilities|Struct|MakeStruct_InventoryItem _itemname_2 _itemid_2 (Math|Integer|Clamp(Integer) (+ (LocalVariables|Getchange_Amount) _itemcount) 0 _maxstack) _maxstack_2 _feedingprogressgain _uiimage _itemactorref _foodtype _staticmesh _meshmaterial _newmeshmaterial))
    ;[1 1 1] Checks to see if more items need to be added into the array
    (if (> (LocalVariables|GetnewCount) _maxstack_2)
      (bind _inventoryitemslots (CallFunction|GetInventoryCount))
      (Utilities|Array|SetArrayElem (Variables|Default|Getinventory) _inventoryitemslots (Utilities|Struct|MakeStruct_InventoryItem (.itemName (Utilities|Struct|BreakStruct_InventoryItem (Utilities|Struct|MakeStruct_InventoryItem _itemname_2 _itemid_2 (Math|Integer|Clamp(Integer) (+ (LocalVariables|Getchange_Amount) _itemcount) 0 _maxstack) _maxstack_2 _feedingprogressgain _uiimage _itemactorref _foodtype _staticmesh _meshmaterial _newmeshmaterial))) (.itemID (Utilities|Struct|BreakStruct_InventoryItem (Utilities|Struct|MakeStruct_InventoryItem _itemname_2 _itemid_2 (Math|Integer|Clamp(Integer) (+ (LocalVariables|Getchange_Amount) _itemcount) 0 _maxstack) _maxstack_2 _feedingprogressgain _uiimage _itemactorref _foodtype _staticmesh _meshmaterial _newmeshmaterial))) (- (LocalVariables|GetnewCount) _maxstack_2) (.maxStack (Utilities|Struct|BreakStruct_InventoryItem (Utilities|Struct|MakeStruct_InventoryItem _itemname_2 _itemid_2 (Math|Integer|Clamp(Integer) (+ (LocalVariables|Getchange_Amount) _itemcount) 0 _maxstack) _maxstack_2 _feedingprogressgain _uiimage _itemactorref _foodtype _staticmesh _meshmaterial _newmeshmaterial))) (.feedingProgressGain (Utilities|Struct|BreakStruct_InventoryItem (Utilities|Struct|MakeStruct_InventoryItem _itemname_2 _itemid_2 (Math|Integer|Clamp(Integer) (+ (LocalVariables|Getchange_Amount) _itemcount) 0 _maxstack) _maxstack_2 _feedingprogressgain _uiimage _itemactorref _foodtype _staticmesh _meshmaterial _newmeshmaterial))) (.UIImage (Utilities|Struct|BreakStruct_InventoryItem (Utilities|Struct|MakeStruct_InventoryItem _itemname_2 _itemid_2 (Math|Integer|Clamp(Integer) (+ (LocalVariables|Getchange_Amount) _itemcount) 0 _maxstack) _maxstack_2 _feedingprogressgain _uiimage _itemactorref _foodtype _staticmesh _meshmaterial _newmeshmaterial))) (.itemActorRef (Utilities|Struct|BreakStruct_InventoryItem (Utilities|Struct|MakeStruct_InventoryItem _itemname_2 _itemid_2 (Math|Integer|Clamp(Integer) (+ (LocalVariables|Getchange_Amount) _itemcount) 0 _maxstack) _maxstack_2 _feedingprogressgain _uiimage _itemactorref _foodtype _staticmesh _meshmaterial _newmeshmaterial))) (.foodType (Utilities|Struct|BreakStruct_InventoryItem (Utilities|Struct|MakeStruct_InventoryItem _itemname_2 _itemid_2 (Math|Integer|Clamp(Integer) (+ (LocalVariables|Getchange_Amount) _itemcount) 0 _maxstack) _maxstack_2 _feedingprogressgain _uiimage _itemactorref _foodtype _staticmesh _meshmaterial _newmeshmaterial))) (.staticMesh (Utilities|Struct|BreakStruct_InventoryItem (Utilities|Struct|MakeStruct_InventoryItem _itemname_2 _itemid_2 (Math|Integer|Clamp(Integer) (+ (LocalVariables|Getchange_Amount) _itemcount) 0 _maxstack) _maxstack_2 _feedingprogressgain _uiimage _itemactorref _foodtype _staticmesh _meshmaterial _newmeshmaterial))) (.meshMaterial (Utilities|Struct|BreakStruct_InventoryItem (Utilities|Struct|MakeStruct_InventoryItem _itemname_2 _itemid_2 (Math|Integer|Clamp(Integer) (+ (LocalVariables|Getchange_Amount) _itemcount) 0 _maxstack) _maxstack_2 _feedingprogressgain _uiimage _itemactorref _foodtype _staticmesh _meshmaterial _newmeshmaterial))) (.newMeshMaterial (Utilities|Struct|BreakStruct_InventoryItem (Utilities|Struct|MakeStruct_InventoryItem _itemname_2 _itemid_2 (Math|Integer|Clamp(Integer) (+ (LocalVariables|Getchange_Amount) _itemcount) 0 _maxstack) _maxstack_2 _feedingprogressgain _uiimage _itemactorref _foodtype _staticmesh _meshmaterial _newmeshmaterial))))))
    (else
      (CallFunction|RemoveInventoryItem itemIndexToChange))))

(fn ReplaceItem
  (params (index :type Integer) (newItem :type Struct%20Inventory%20Item%20Structure))
  ;[1 1 1] Replaces the inventory item in the array position
  (bind (_index _found) (CallFunction|FindIteminInventory newItem)) ; Searches inventory for the item
  (if _found ; If item has been found
    ;;[1 0 0] Stacks the items if it already exists in the inventory
    (CallFunction|ItemCountChange _index newItem true)
    (else
      (Utilities|Array|SetArrayElem (Variables|Default|Getinventory) index newItem))))

(fn RemoveInventoryItem
  (params (index :type Integer))
  ;[1 1 1] Removes an item from the inventory
  (Utilities|Array|SetArrayElem (Variables|Default|Getinventory) index (Utilities|Struct|MakeStruct_InventoryItem "Item" 0 0 20 1e+01 0 "/Game/t014172k/Blueprints/Items/BP_PickupItem.BP_PickupItem_C")) ; Sets the array element to the\ndefault (empty) struct
)

(fn IsInventoryFull
  (bind _inventoryitemslots (CallFunction|GetInventoryCount)) ; Gets the inventory item count and checks if it matches the max slots
  (return (>= _inventoryitemslots (Variables|Default|GetinventorySlots))))

(fn GetInventoryCount
  ;[1 1 1] Loops through each inventory item, and checks to see if the ID is not equal to 0 (empty)
  (for _array_element (Variables|Default|Getinventory)
    (if (not (== (.itemID (Utilities|Struct|BreakStruct_InventoryItem _array_element)) 0))
      (Math|Integer|IncrementInt (LocalVariables|Getitem_Count))))
  (return (LocalVariables|Getitem_Count)))

(fn SwapEquippedItem
  (params (isIncreasing :type Boolean))
  ;[1 1 1] Checks to make sure there is more than 1 item in the inventory
  (bind _inventoryitemslots (CallFunction|GetInventoryCount))
  (bind _output_get (LocalVariables|SetinvLength _inventoryitemslots))
  (if (> _output_get 0)
    ;[1 1 1] Updates the held item index and then the display
    ;;[1 0 0] Changes held item index value
    (if isIncreasing
      (bind _result (Math|Integer|IncrementInt (Variables|Default|GetheldItemIndex))
        (:%20%20
          ;;[1 0 0] Error checks to make sure the values haven't exceeded the inventory
          (if (>= _result (LocalVariables|GetinvLength))
            (Variables|Default|SetheldItemIndex 0))))
      (else
        (bind _result_2 (Math|Integer|DecrementInt (Variables|Default|GetheldItemIndex))
          (:%20%20
            (if (< _result_2 0)
              (Variables|Default|SetheldItemIndex (- (LocalVariables|GetinvLength) 1)))))))
    (CallFunction|UpdateHeldItem)))

(fn SortInventory
  ;[1 1 1] Loops through the inventory and gets all the slots that have items in them
  (for _index (range 0 (- (Variables|Default|GetinventorySlots) 1))
    (if (!= (.itemID (Utilities|Struct|BreakStruct_InventoryItem (Utilities|Array|Get(acopy) (Variables|Default|Getinventory) _index))) 0)
      (Utilities|Array|Add (LocalVariables|Getnew_Inventory) (Utilities|Array|Get(acopy) (Variables|Default|Getinventory) _index))))
  ;[1 1 1] While new_Inventory.Length < inventorySlots
  (while (< (Utilities|Array|Length (LocalVariables|Getnew_Inventory)) (Variables|Default|GetinventorySlots))
    ;[1 1 1] Fills up the rest of the inventory with empty item slots
    (Utilities|Array|Add (LocalVariables|Getnew_Inventory) (Utilities|Struct|MakeStruct_InventoryItem "Item" 0 0 20 1e+01 0 "/Game/t014172k/Blueprints/Items/BP_PickupItem.BP_PickupItem_C")))
  ;[1 1 1] Sets the inventory to the newly
  ; sorted array
  (Variables|Default|Setinventory (LocalVariables|Getnew_Inventory)))

(fn GetInventory
  (return (Variables|Default|Getinventory)))

(fn UpdateHeldItem
  (Class|BPIPlayer|IUpdateHeldItem(Message) (Components|GetOwner) (Utilities|Array|Get(acopy) (Variables|Default|Getinventory) (Variables|Default|GetheldItemIndex))))

(fn GetItem
  (params (index :type Integer))
  (return (Utilities|Array|Get(acopy) (Variables|Default|Getinventory) index)))

(fn ItemUsed
  (CallFunction|ItemCountChange (Variables|Default|GetheldItemIndex) (Utilities|Struct|MakeStruct_InventoryItem "Item" 0 1 20 1e+01 0 0) false))

(fn SortInventoryStacks
  (params (IDToCheck :type Integer))
  (for (_array_element _array_index) (Variables|Default|Getinventory)
    (if (== (.itemID (Utilities|Struct|BreakStruct_InventoryItem _array_element)) IDToCheck)
      (for (_array_element_2 _array_index_2) (Variables|Default|Getinventory)
        (if (and (== (.itemID (Utilities|Struct|BreakStruct_InventoryItem _array_element_2)) IDToCheck) (!= _array_index_2 _array_index))
          (CallFunction|ItemCountChange _array_index _array_element_2 true)
          (CallFunction|RemoveInventoryItem _array_index_2))))))

(fn SetHeldItem
  (params (index :type Integer))
  ;[1 1 1] Checks to make sure the selected index is within the bounds of the inventory
  (bind _inventoryitemslots (CallFunction|GetInventoryCount))
  (if (and (>= _inventoryitemslots index) (>= index 0))
    ;[1 1 1] Sets the new held item index and updates the display
    (Variables|Default|SetheldItemIndex index)
    (CallFunction|UpdateHeldItem)))

(fn ClearInventory
  ;[1 1 1] Clears each item out of the inventory
  (for (_ _array_index) (Variables|Default|Getinventory)
    (CallFunction|RemoveInventoryItem _array_index))
  (CallFunction|UpdateHeldItem))

(fn GetStarCount
  ;[1 1 1] Gets the amount of stars that are in the player's inventory
  (for _array_element (Variables|Default|Getinventory)
    (if (Utilities|Enum|Equal(Enum) (.foodType (Utilities|Struct|BreakStruct_InventoryItem _array_element)) "NewEnumerator4")
      (LocalVariables|SetstarCount (+ (.itemCount (Utilities|Struct|BreakStruct_InventoryItem _array_element)) (LocalVariables|GetstarCount)))))
  (return (LocalVariables|GetstarCount)))