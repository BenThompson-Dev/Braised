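; Shed actor that acts as an interactable storage container, letting the player move items between their inventory and the shed's.
; On init it creates a hidden storage menu widget; interacting shows it, switches to UI-only input and stops player movement.
; Item swaps go through inventory interface messages sent to either the shed or player, chosen by an in-storage flag.
; The shed's inventory component is then sorted and both displays refresh.
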(event Custom|SwapInventoryItems
  (params (item1_ID :type Integer) (item1_isInStorage :type Boolean) (item2_ID :type Integer) (item2_isInStorage :type Boolean))
  ;[1 1 1] Moves the items when two have been selected
  (CallFunction|SwapItems item1_ID item1_isInStorage item2_ID item2_isInStorage)
  (Default|SortInventory (Variables|Default|GetBPC_Inventory))
  (CallFunction|UpdateUI))

(event Custom|UpdateUI
  ;[1 1 1] Updates all the UI elements to reflect the current inventory and storage
  (bind _inventory (Class|BPIInventory|IGetInv(Message) (Variables|Default|GetPlayer%20Ref)))
  (bind _inventory_2 (Default|GetInventory (Variables|Default|GetBPC_Inventory)))
  (Default|UpdateUI (Variables|Default|GetmenuUI) _inventory_2 _inventory))

(event EventISetItem
  (params (itemID :type Integer) (newItem :type Struct%20Inventory%20Item%20Structure))
  ;[1 1 1] Sets the item in the inventory
  (Default|ReplaceItem (Variables|Default|GetBPC_Inventory) itemID newItem))

(event EventIInit
  ;[1 1 1] Sets up storage menu widget
  (bind _returnvalue (UserInterface|CreateWidget "/Game/t014172k/UI/UI_StorageInventory.UI_StorageInventory_C"))
  (bind _output_get (Variables|Default|SetmenuUI _returnvalue))
  (UserInterface|Viewport|AddtoViewport _output_get 0)
  (Widget|SetVisibility _output_get "Hidden")
  (Default|SetUpUI _output_get)
  (EventDispatchers|BindEventtoSwapItems (Variables|Default|GetmenuUI) (delegate Custom|SwapInventoryItems))
  (Default|IInit (Variables|Default|GetBPC_Inventory)))

(event EventISortInv
  (params (index :type Integer))
  ;[1 1 1] Sorts the inventory
  (Default|SortInventoryStacks (Variables|Default|GetBPC_Inventory) index))

(event EventIInteract
  (params (playerRef :type Character%20Object%20Reference))
  (bind _returnvalue (Game|GetPlayerController 0))
  ;[1 1 1] Handles opening the UI menu
  (Variables|Default|SetPlayer%20Ref playerRef)
  (Input|SetInputModeUIOnly _returnvalue (Variables|Default|GetmenuUI) "DoNotLock")
  (Variables|/Script/Engine.PlayerController|SetbShowMouseCursor _returnvalue true)
  (Widget|SetVisibility (Variables|Default|GetmenuUI) "Visible")
  (Class|BPIPlayer|ISetCanMove(Message) playerRef false) ; Changes player movement state
  (CallFunction|UpdateUI)
  (Default|CallShedOpened))

(event EventIRemoveItem
  (params (index :type Integer))
  (Default|RemoveInventoryItem (Variables|Default|GetBPC_Inventory) index))

(fn ConstructionScript)

(fn SwapItems
  (params (item1_ID :type Integer) (item1_invRef :type Boolean) (item2_ID :type Integer) (item2_invRef :type Boolean))
  (bind _actorref (CallFunction|GetCorrectInventory item1_invRef))
  (LocalVariables|Setitem_1_Actor_Ref _actorref)
  (bind _actorref_2 (CallFunction|GetCorrectInventory item2_invRef))
  (LocalVariables|Setitem_2_Actor_Ref _actorref_2)
  ;[1 1 1] Gets both of the items
  (bind _item (Class|BPIInventory|IGetItem(Message) (LocalVariables|Getitem_1_Actor_Ref) item1_ID))
  (LocalVariables|Setitem_1 _item)
  (bind _item_2 (Class|BPIInventory|IGetItem(Message) (LocalVariables|Getitem_2_Actor_Ref) item2_ID))
  (LocalVariables|Setitem_2 _item_2)
  (Class|BPIInventory|IRemoveItem(Message) (LocalVariables|Getitem_1_Actor_Ref) item1_ID)
  (Class|BPIInventory|IRemoveItem(Message) (LocalVariables|Getitem_2_Actor_Ref) item2_ID)
  ;[1 1 1] Sets the items in the inventories
  (Class|BPIInventory|ISetItem(Message) (LocalVariables|Getitem_1_Actor_Ref) item1_ID (LocalVariables|Getitem_2))
  (Class|BPIInventory|ISetItem(Message) (LocalVariables|Getitem_2_Actor_Ref) item2_ID (LocalVariables|Getitem_1)))

(fn GetCorrectInventory
  (params (isInStorage :type Boolean))
  (if isInStorage
    (LocalVariables|Setactor self)
    (else
      (LocalVariables|Setactor (Variables|Default|GetPlayer%20Ref))))
  (return (LocalVariables|Getactor)))

(fn IGetInv
  ;[1 1 1] Returns the inventory
  (bind _inventory (Default|GetInventory (Variables|Default|GetBPC_Inventory)))
  (return _inventory))

(fn IGetItem
  (params (itemIndex :type Integer))
  (bind _item (Default|GetItem (Variables|Default|GetBPC_Inventory) itemIndex))
  (return _item))