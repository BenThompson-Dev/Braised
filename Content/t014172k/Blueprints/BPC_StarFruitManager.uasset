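; Manager component that spawns star fruit pickups at every star spawn point on init and respawns a requested count.
; Each fruit carries its spawn index and reports pickup through a dispatcher, which queues that index as removed.
; Respawning consumes queued indices oldest first, falling back to a search of spawn-point in-use flags.
; A bound shed's opened event clears the queue.
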(event Custom|SpawnFruit
  (params (spawnPoint :type Actor%20Object%20Reference) (index :type Integer))
  ;[1 1 1] Spawns a fruit at a given spawn point
  (bind _returnvalue (Game|SpawnActorfromClass "/Game/b014818k/Blueprints/BP_FoodPickUpStar.BP_FoodPickUpStar_C" (Transformation|GetActorTransform spawnPoint) "AlwaysSpawn" 0 0))
  (Default|IInit _returnvalue)
  (Default|ISetSpawnIndex _returnvalue index)
  (EventDispatchers|BindEventtoStarPickedUp _returnvalue (delegate Custom|StarPickedUp)) ; Adds listener to pick up event
  (Class|BPIStar|ISetIsinUse(Message) spawnPoint true))

(event Custom|RespawnFruits
  (params (count :type Integer))
  (bind _removedstarfruits (Variables|Default|GetremovedStarFruits))
  (bind _output (Utilities|Array|Get(acopy) _removedstarfruits))
  ;[1 1 1] Handles respawning the fruits when needed
  (for _index (range 0 (- count 1))
    ;;[1 0 0] Checks if the removed stars array has values in it
    (if (> (Utilities|Array|Length (Variables|Default|GetremovedStarFruits)) 0)
      ;;[1 0 0] Uses the first index of the removed star fruit array as a spawn point
      (CallFunction|SpawnFruit (Utilities|Array|Get(acopy) (Variables|Default|GetspawnPoints) _output) _output)
      (Utilities|Array|RemoveIndex (Variables|Default|GetremovedStarFruits))
      (else
        ;;[1 0 0] Gets the unused point and respawns the fruit at it
        (bind _foundindex (CallFunction|GetUnusedSpawnPoint))
        (CallFunction|SpawnFruit (Utilities|Array|Get(acopy) (Variables|Default|GetspawnPoints) _foundindex) _foundindex)))))

(event Custom|StarPickedUp
  (params (starIndex :type Integer))
  ;[1 1 1] Handles adding the star to the removed array and setting the spawn point to not be in use
  (Development|PrintString "picked up")
  (bind _returnvalue (Utilities|Array|Add (Variables|Default|GetremovedStarFruits) starIndex))
  (Class|BPIStar|ISetIsinUse(Message) (Utilities|Array|Get(acopy) (Variables|Default|GetspawnPoints) _returnvalue) false))

(event Custom|EventBinding
  (params (shed :type BP%20Shed%20Object%20Reference))
  ;[1 1 1] Sets up the event dispatcher binding
  (EventDispatchers|BindEventtoShedOpened shed (delegate Custom|ClearHeldStars)))

(event Custom|ClearHeldStars
  ;[1 1 1] Sets up the event dispatcher binding
  (Utilities|Array|Clear (Variables|Default|GetremovedStarFruits)))

(event EventIInit
  ;[1 1 1] Spawns all the fruit when initialised
  (bind _outactors (Actor|GetAllActorsOfClass "/Game/t014172k/Blueprints/BP_StarSpawnPoint.BP_StarSpawnPoint_C"))
  (bind _output_get (Variables|Default|SetspawnPoints _outactors))
  (for (_array_element _array_index) _output_get
    (CallFunction|SpawnFruit _array_element _array_index)))

(fn GetUnusedSpawnPoint
  ;[1 1 1] Finds the first star spawn point in the array that is not in use
  (bind (_array_element _array_index) (Utilities|Array|ForEachLoopwithBreak (Variables|Default|GetspawnPoints) :!label _label)
    (:LoopBody
      (LocalVariables|SetcurrentIndex _array_index)
      (bind _isinuse (Class|BPIStar|IGetIsinUse(Message) _array_element))
      (if _isinuse
        (goto _label Break)))
    (:Completed
      (return (LocalVariables|GetcurrentIndex)))))