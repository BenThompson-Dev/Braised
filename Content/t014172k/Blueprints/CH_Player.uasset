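; First-person player character, driven mostly by interface events for movement, health and respawn, inventory and held items, menus and music.
; BPCInventory feeds the player UI and the item actor attached to the hand.
; Camera line traces send interact and release messages, with looping timers updating crosshair prompts and hold-to-release progress for creatures (Motes).
; Death reports the star count to the game mode, clears the inventory and returns to PlayerStart.
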(event Custom|ReleaseTimer
  (bind _playerui (Variables|Default|GetplayerUI))
  (bind _firstpersoncamera (Variables|Default|GetFirstPersonCamera))
  (bind _playerui_2 (Variables|Default|GetplayerUI))
  (bind _playerui_3 (Variables|Default|GetplayerUI))
  (bind _returnvalue (Transformation|GetWorldLocation _firstpersoncamera))
  (if (Variables|Default|GetinteractOn)
    ;[1 1 1] b014818k - Fires off a linetrace where the player is looking
    (bind (_outhit _returnvalue_2) (Collision|LineTraceByChannel _returnvalue (+ _returnvalue (* (Math|Vector|GetForwardVector _firstpersoncamera) (Variables|Default|GetuseTraceLength))) "TraceTypeQuery2" false 0 "None"))
    (if _returnvalue_2
      ;[1 1 1] b014818k - Get the creature reference and check if it exists, in case it is destroyed.
      (bind _creaturereference (Class|BPIBaseCreature|IGetCreatureReference(Message) (.HitActor (Collision|BreakHitResult _outhit)) true))
      (Utilities|IsValid _creaturereference
        (:Is%20Valid
          (if (== _creaturereference (.HitActor (Collision|BreakHitResult _outhit)))
            ;[1 1 1] b014818k - Update the timer
            (bind _output_get (Variables|Default|SetreleaseTime (+ (Variables|Default|GetreleaseTime) 0.05)))
            ;[1 1 1] b014818k - If the timer has reached above 1, call the final release creature.
            (Default|UpdateReleaseProgress (Variables|Default|GetplayerUI) _output_get)
            (if (>= (+ (Variables|Default|GetreleaseTime) 0.05) 1.2)
              (Class|BPIBaseCreature|IReleaseCreatureFinal(Message) _creaturereference))
            (else
              ;[1 1 1] b014818k - If the hit target isn't the creature, clear the timer.
              (bind _output_get_2 (Variables|Default|SetreleaseTime 0.0))
              (Default|UpdateReleaseProgress _playerui_2 _output_get_2)
              (Default|HideReleaseProgress _playerui_2 true)))))
      (else
        ;[1 1 1] b014818k - If there wasn't a hit, clear the timer.
        (bind _output_get_3 (Variables|Default|SetreleaseTime 0.0))
        (Default|UpdateReleaseProgress _playerui_3 _output_get_3)
        (Default|HideReleaseProgress _playerui_3 true)))
    (else
      ;[1 1 1] b014818k - Clears the timer and the time if the player isn't holding M1.
      (Utilities|Time|ClearandInvalidateTimerbyHandle (Variables|Default|GetreleaseTimerHandle))
      (bind _output_get_4 (Variables|Default|SetreleaseTime 0.0))
      (Default|UpdateReleaseProgress _playerui _output_get_4)
      (Default|HideReleaseProgress _playerui true))))

(event Custom|ResetPlayer
  (bind _spawnpoint (Variables|Default|GetspawnPoint))
  ;[1 1 1] t014172k - Resets the player if they die
  (bind _inventorystarcount (Default|GetStarCount (Variables|Default|GetBPC_Inventory))) ; Gets the amount of stars in the player's inventory when\nthey died
  (Class|BPIGM|IRespawnFruits(Message) (Game|GetGameMode) _inventorystarcount)
  (Default|ClearInventory (Variables|Default|GetBPC_Inventory))
  (bind _inventory (Default|GetInventory (Variables|Default|GetBPC_Inventory)))
  (Default|UpdateUI (Variables|Default|GetplayerUI) _inventory)
  (Transformation|SetActorLocation (Transformation|GetActorLocation _spawnpoint) false false)
  (Transformation|SetActorRotation (Transformation|GetActorRotation _spawnpoint))
  (Variables|Default|SetHealth 1e+02))

(event Custom|PopUpUI
  (params (item :type Struct%20Inventory%20Item%20Structure) (enum :type PopupType%20Enum :default "NewEnumerator0") (Creature%20level :type Integer))
  (bind _playerui (Variables|Default|GetplayerUI))
  (bind _playerui_2 (Variables|Default|GetplayerUI))
  (bind _popup (Variables|/Game/t014172k/UI/UI_PlayerUI.UI_PlayerUI_C|GetPopup _playerui_2))
  (bind _popup_2 (Variables|/Game/t014172k/UI/UI_PlayerUI.UI_PlayerUI_C|GetPopup _playerui))
  (bind _textblock_23 (Variables|/Game/r012966j__Jake_/UI/Popup.Popup_C|GetTextBlock_23 _popup_2))
  ;[1 1 1] r012966j Popup UI
  (Utilities|FlowControl|Sequence
    (:then_0
      (switch Utilities|FlowControl|Switch|SwitchonPopupType enum
        (:NewEnumerator0)
        (:NewEnumerator1
          (Rendering|Components|TextRender|SetText _textblock_23 "Mote teleported!"))
        (:NewEnumerator2
          (Rendering|Components|TextRender|SetText _textblock_23 (Utilities|Text|ToText(String) (Utilities|String|Append "Mote level " (Utilities|String|ToString(Integer) Creature%20level)))))
        (:NewEnumerator3
          (Rendering|Components|TextRender|SetText _textblock_23 "You have released your Mote!"))
        (:NewEnumerator4
          (Rendering|Components|TextRender|SetText _textblock_23 "Mote already at max level, hold Q to release!"))
        (:NewEnumerator5
          (Audio|PlaySound2D "/Game/W015955i_WillW/Audio/Motes/S_MoteEvolve.S_MoteEvolve" 1.0 1.0 0.0 0 0)
          (Rendering|Components|TextRender|SetText _textblock_23 "More information has been added to the journal!"))))
    (:then_1
      (Widget|SetVisibility _popup "Visible")
      (Utilities|FlowControl|Delay 4.0)
      (Widget|SetVisibility _popup "Hidden"))))

(event Custom|CrosshairInteract
  (bind _firstpersoncamera (Variables|Default|GetFirstPersonCamera))
  (bind _playerui (Variables|Default|GetplayerUI))
  (bind _playerui_2 (Variables|Default|GetplayerUI))
  (bind _playerui_3 (Variables|Default|GetplayerUI))
  (bind _returnvalue (Transformation|GetWorldLocation _firstpersoncamera))
  (bind _ui_crosshair2 (Variables|/Game/t014172k/UI/UI_PlayerUI.UI_PlayerUI_C|GetUI_Crosshair2 _playerui_2))
  (bind _ui_crosshair (Variables|/Game/t014172k/UI/UI_PlayerUI.UI_PlayerUI_C|GetUI_Crosshair _playerui_3))
  ;[1 1 1] b014818k - Crosshair colour changing
  (bind (_outhit _returnvalue_2) (Collision|LineTraceByChannel _returnvalue (+ _returnvalue (* (Math|Vector|GetForwardVector _firstpersoncamera) (Variables|Default|GetuseTraceLength))) "TraceTypeQuery2" false 0 "None"))
  (if _returnvalue_2
    (bind (_caninteract _interacttext) (Class|BPIInteract|ICanInteract(Message) (.HitActor (Collision|BreakHitResult _outhit))))
    (if _caninteract
      (Widget|SetVisibility _ui_crosshair "Hidden")
      (Widget|SetVisibility _ui_crosshair2 "Visible")
      (switch Utilities|FlowControl|Switch|SwitchonEnum_InteractText _interacttext
        (:NewEnumerator0
          (Widget|SetVisibility (Variables|/Game/t014172k/UI/UI_PlayerUI.UI_PlayerUI_C|GetUI_InteractE _playerui) "Visible"))
        (:NewEnumerator1
          (Widget|SetVisibility (Variables|/Game/t014172k/UI/UI_PlayerUI.UI_PlayerUI_C|GetUI_UseItem _playerui) "Visible"))
        (:NewEnumerator2
          (Widget|SetVisibility (Variables|/Game/t014172k/UI/UI_PlayerUI.UI_PlayerUI_C|GetUI_Release _playerui) "Visible")))
      (else
        (Widget|SetVisibility _ui_crosshair "Visible" :!label _label)
        (Widget|SetVisibility _ui_crosshair2 "Hidden")
        (switch Utilities|FlowControl|Switch|SwitchonEnum_InteractText _interacttext
          (:NewEnumerator0
            (Widget|SetVisibility (Variables|/Game/t014172k/UI/UI_PlayerUI.UI_PlayerUI_C|GetUI_InteractE _playerui) "Hidden"))
          (:NewEnumerator1
            (Widget|SetVisibility (Variables|/Game/t014172k/UI/UI_PlayerUI.UI_PlayerUI_C|GetUI_UseItem _playerui) "Hidden"))
          (:NewEnumerator2
            (Widget|SetVisibility (Variables|/Game/t014172k/UI/UI_PlayerUI.UI_PlayerUI_C|GetUI_Release _playerui) "Hidden")))))
    (else
      (goto _label))))

(event EventISwapHeldItem
  (params (isIncreasing :type Boolean))
  ;[1 1 1] Swaps the player's held item
  (Default|SwapEquippedItem (Variables|Default|GetBPC_Inventory) isIncreasing))

(event EventIAddItem
  (params (addItem :type Struct%20Inventory%20Item%20Structure) (itemRef :type Actor%20Object%20Reference))
  (bind _bpc_inventory (Variables|Default|GetBPC_Inventory))
  ;[1 1 1] t014172k - Handles picking up items
  (Default|AddItem _bpc_inventory addItem itemRef)
  (bind _inventory (Default|GetInventory _bpc_inventory))
  (Default|UpdateUI (Variables|Default|GetplayerUI) _inventory)
  (CallFunction|PopUpUI addItem "NewEnumerator0"))

(event EventISetCanMove
  (params (canMove :type Boolean))
  (bind _returnvalue (Game|GetPlayerController 0))
  ;[1 1 1] Changes the player's move state (used to stop movement when UI is on screen)
  (bind _output_get (Variables|Default|SetcanMove canMove))
  (Input|SetIgnoreMoveInput _returnvalue (not _output_get))
  (Input|SetIgnoreLookInput _returnvalue (not _output_get))
  (if (not (Variables|Default|GetcanMove))
    (Variables|/Script/Engine.MovementComponent|SetVelocity (Variables|Character|GetCharacterMovement) "0, 0, 0") ; Cancels velocity
  ))

(event EventISetItem
  (params (itemID :type Integer) (newItem :type Struct%20Inventory%20Item%20Structure))
  ;[1 1 1] Sets the new item in the inventory
  (Default|ReplaceItem (Variables|Default|GetBPC_Inventory) itemID newItem))

(event EventIUpdateInventoryDisplay
  (bind _bpc_inventory (Variables|Default|GetBPC_Inventory))
  ;[1 1 1] t014172k - Updates the player's inventory display and held item (for when they exit the storage menu)
  (Default|SortInventory (Variables|Default|GetBPC_Inventory))
  (bind _inventory (Default|GetInventory _bpc_inventory))
  (Default|UpdateUI (Variables|Default|GetplayerUI) _inventory)
  (Default|UpdateHeldItem _bpc_inventory))

(event EventIShowTeleportMap
  (params (creatureToTeleport :type Actor%20Object%20Reference))
  (Default|ShowUI (Variables|Default|GetteleportUIMap) creatureToTeleport))

(event EventIItemUse
  (bind _helditemref (Variables|Default|GetheldItemRef))
  ;[1 1 1] t014172k - Handles using the current item
  (Utilities|IsValid _helditemref
    (:Is%20Valid
      (bind _succeeded (Class|BPIItem|IUse(Message) _helditemref (Variables|Default|GetFirstPersonCamera)))
      (if _succeeded
        (Default|ItemUsed (Variables|Default|GetBPC_Inventory))
        (CallFunction|IUpdateInventoryDisplay)))))

(event EventICallDestroyItem
  (Default|CallDestroyItem))

(event EventIInit
  (Variables|Default|SetJumpMaxCount 1)
  (Default|IInit (Variables|Default|GetBPC_Inventory))
  ;[1 1 1] Sets up the player UI
  (bind _returnvalue (UserInterface|CreateWidget "/Game/t014172k/UI/UI_PlayerUI.UI_PlayerUI_C"))
  (bind _output_get (Variables|Default|SetplayerUI _returnvalue))
  (UserInterface|Viewport|AddtoViewport _output_get 0)
  (bind _inventory (Default|GetInventory (Variables|Default|GetBPC_Inventory)))
  (Default|SetUpUI (Variables|Default|GetplayerUI) _inventory)
  ;[1 1 1] Stores the player spawn point
  (bind _returnvalue_2 (Actor|GetActorOfClass "/Script/Engine.PlayerStart"))
  (Variables|Default|SetspawnPoint _returnvalue_2)
  ;[1 1 1] Initialises the music manager
  (bind _returnvalue_3 (Game|SpawnActorfromClass "/Game/t014172k/Blueprints/BP_MusicManager.BP_MusicManager_C" (Math|Transform|MakeTransform "0, 0, 0") "Undefined" 0 0))
  (bind _output_get_2 (Variables|Default|SetmusicManager _returnvalue_3))
  (Class|BPIInit|IInit(Message) _output_get_2)
  (bind _returnvalue_4 (UserInterface|CreateWidget "/Game/w027457k/UI/UITESTS/UI_PauseMenu.UI_PauseMenu_C"))
  (Variables|Default|SetPauseMenuREF _returnvalue_4)
  (Utilities|Time|SetTimerbyFunctionName 0 "CrosshairInteract" 0.1 true)
  (Variables|Default|SetdefaultCrosshairColour (Variables|/Script/UMG.Image|GetColorAndOpacity (Variables|/Game/w027457k/UI/UITESTS/UI_Crosshair.UI_Crosshair_C|GetCrosshairImage (Variables|/Game/t014172k/UI/UI_PlayerUI.UI_PlayerUI_C|GetUI_Crosshair (Variables|Default|GetplayerUI)))))
  (Variables|Default|SetisHolding false))

(event EventISortInv
  (params (index :type Integer))
  (Default|SortInventoryStacks (Variables|Default|GetBPC_Inventory) index))

(event EventIRemoveItem
  (params (index :type Integer))
  (Default|RemoveInventoryItem (Variables|Default|GetBPC_Inventory) index))

(event EventIJump
  ;[1 1 1] Movement inputs
  (Character|Jump))

(event EventIToolInteract
  (bind _self self)
  (bind _firstpersoncamera (Variables|Default|GetFirstPersonCamera))
  (bind _returnvalue (Transformation|GetWorldLocation _firstpersoncamera))
  ;[1 1 1] t014172k - Interact tool functionality
  (bind (_outhit _returnvalue_2) (Collision|LineTraceByChannel _returnvalue (+ _returnvalue (* (Math|Vector|GetForwardVector _firstpersoncamera) (Variables|Default|GetuseTraceLength))) "TraceTypeQuery2" false 0 "None"))
  (if _returnvalue_2
    (EventDispatchers|UnbindallEventsfromDestroyItem) ; Unbinds all listeners to the event so that multiple\nobjects aren't potentially destroyed
    (Class|BPIInteract|IInteract(Message) (.HitActor (Collision|BreakHitResult _outhit)) _self _self)
    (else
      (Development|PrintString "no objects hit"))))

(event EventIStackItems
  (params (baseItem :type Struct%20Inventory%20Item%20Structure) (itemToAdd :type Struct%20Inventory%20Item%20Structure))
  ;[1 1 1] Finds the base item in the inventory and stacks the new item on top
  (bind (_index _found) (Default|FindIteminInventory (Variables|Default|GetBPC_Inventory) baseItem))
  (if _found
    (Default|ItemCountChange (Variables|Default|GetBPC_Inventory) _index itemToAdd true)))

(event EventISetTeleportMapUI
  (params (Map :type UI%20Map%20Object%20Reference))
  ;[1 1 1] b014818k - Sets up the creature teleporting map
  (Variables|Default|SetteleportUIMap Map))

(event EventIReleaseCreature
  ;[1 1 1] b014818k - Starts release creature timer
  (bind _returnvalue (Utilities|Time|SetTimerbyEvent (delegate Custom|ReleaseTimer) 0.05 true))
  (Variables|Default|SetreleaseTimerHandle _returnvalue))

(event EventISetHealth
  (params (UpdatedHealth :type Float%20%28single-precision%29))
  ;[1 1 1] Adds Set Health Function using Interface - l014519j
  (Variables|Default|SetHealth UpdatedHealth))

(event EventIUpdateMusic
  (params (newTrack :type Enum_Music%20Enum :default "NewEnumerator0"))
  ;[1 1 1] Music manager interface functions
  (Class|BPIMusic|ISetSound(Message) (Variables|Default|GetmusicManager) newTrack))

(event EventIDarknessMusic
  (params (isActive :type Boolean))
  ;[1 1 1] Music manager interface functions
  (Class|BPIMusic|ISetDarknessMusic(Message) (Variables|Default|GetmusicManager) isActive))

(event EventISprint
  (params (Start :type Boolean))
  ;[1 1 1] b014818k - Sprint
  (if Start
    (Variables|/Script/Engine.CharacterMovementComponent|SetMaxWalkSpeed (Variables|Character|GetCharacterMovement) 9e+02)
    (else
      (Variables|/Script/Engine.CharacterMovementComponent|SetMaxWalkSpeed (Variables|Character|GetCharacterMovement) 6e+02))))

(event EventITryRelease
  (bind _self self)
  (bind _firstpersoncamera (Variables|Default|GetFirstPersonCamera))
  (bind _returnvalue (Transformation|GetWorldLocation _firstpersoncamera))
  ;[1 1 1] t014172k - Starts trying to release a creature in a pen
  (Variables|Default|SetinteractOn true)
  (bind (_outhit _returnvalue_2) (Collision|LineTraceByChannel _returnvalue (+ _returnvalue (* (Math|Vector|GetForwardVector _firstpersoncamera) (Variables|Default|GetuseTraceLength))) "TraceTypeQuery2" false 0 "None"))
  (if _returnvalue_2
    (EventDispatchers|UnbindallEventsfromDestroyItem) ; Unbinds all listeners to the event so that multiple\nobjects aren't potentially destroyed
    (Class|BPIInteract|IRelease(Message) (.HitActor (Collision|BreakHitResult _outhit)) _self _self)
    (else
      (Development|PrintString "no objects hit"))))

(event EventIReleaseEnd
  ;[1 1 1] t014172k - Starts trying to release a creature in a pen
  (Variables|Default|SetinteractOn false))

(event EventIMoveForward
  (params (axisAmount :type Float%20%28single-precision%29))
  ;[1 1 1] Movement inputs
  (Pawn|Input|AddMovementInput (Transformation|GetActorForwardVector) axisAmount false))

(event EventIInteractStart
  ;[1 1 1] t014172k - Interact tool functionality
  (Default|CallInteractUse))

(event EventIMoveRight
  (params (axisAmount :type Float%20%28single-precision%29))
  ;[1 1 1] Movement inputs
  (Pawn|Input|AddMovementInput (Transformation|GetActorRightVector) axisAmount false))

(event EventISetHeldItem
  (params (index :type Integer))
  ;[1 1 1] Swaps the player's held item
  (Default|SetHeldItem (Variables|Default|GetBPC_Inventory) index))

(event EventITurn
  (params (axisAmount :type Float%20%28single-precision%29))
  ;[1 1 1] Mouse direction input
  (Pawn|Input|AddControllerYawInput axisAmount))

(event EventILookUp
  (params (axisAmount :type Float%20%28single-precision%29))
  ;[1 1 1] Mouse direction input
  (Pawn|Input|AddControllerPitchInput axisAmount))

(event EventTakeDamage
  (params (Damage :type Float%20%28single-precision%29))
  ;[1 1 1] Health System - l014519j
  (bind _output_get (Variables|Default|SetHealth (- (Variables|Default|GetHealth) Damage)))
  (Development|PrintString (Utilities|String|ToString(Float) _output_get))
  (if (<= (Variables|Default|GetHealth) 0.0)
    (CallFunction|ResetPlayer)))

(event EventIUpdateHeldItem
  (params (item :type Struct%20Inventory%20Item%20Structure))
  (bind (_itemname _itemid _itemcount _maxstack _feedingprogressgain _uiimage _itemactorref) (Utilities|Struct|BreakStruct_InventoryItem item))
  (bind (_itemname_2 _itemid_2 _itemcount_2 _maxstack_2 _feedingprogressgain_2 _uiimage_2 _itemactorref_2 _foodtype _staticmesh _meshmaterial _newmeshmaterial _heldmesh _heldrotation) (Utilities|Struct|BreakStruct_InventoryItem item))
  ;[1 1 1] t014172k - Updates the held item mesh
  (Utilities|IsValid (Variables|Default|GetheldItemRef) ; If a held item is already in the world
    (:Is%20Valid
      (Actor|DestroyActor (Variables|Default|GetheldItemRef)))
    (:Is%20Not%20Valid
      _))
  (bind _output_get (Variables|Default|SetisHolding (!= _itemid 0)))
  (if _output_get
    (bind _returnvalue (Game|SpawnActorfromClass _itemactorref (Math|Transform|MakeTransform "0, 0, 0" _heldrotation "10.000000,10.000000,10.000000") "Undefined" 0 0))
    (Class|BPIItem|ISetData(Message) _returnvalue (Utilities|Struct|MakeStruct_InventoryItem _itemname_2 _itemid_2 1 _maxstack_2 _feedingprogressgain_2 _uiimage_2 _itemactorref_2 _foodtype _staticmesh _meshmaterial _newmeshmaterial _heldmesh _heldrotation))
    (bind _output_get_2 (Variables|Default|SetheldItemRef _returnvalue))
    (Class|BPIItem|IHold(Message) _output_get_2)
    (Transformation|AttachComponentToComponent _output_get_2 (Variables|Default|GetRightHand) "HandSocket" "KeepRelative" "KeepRelative" "KeepWorld" true)))

(event Input|ActionEvents|InputActionPauseButton
  (params (Key :type Key%20Structure :default "None"))
  (bind _returnvalue (Game|GetPlayerController 0))
  (bind _pausemenuref (Variables|Default|GetPauseMenuREF))
  ;[1 1 1] Creates Pause Menu
  (:Pressed
    (if (Game|IsGamePaused)
      (Widget|RemovefromParent _pausemenuref)
      (Game|SetGamePaused false)
      (Variables|/Script/Engine.PlayerController|SetbShowMouseCursor _returnvalue false)
      (Input|SetInputModeGameOnly _returnvalue)
      (else
        (UserInterface|Viewport|AddtoViewport _pausemenuref 0)
        (Game|SetGamePaused true)
        (Variables|/Script/Engine.PlayerController|SetbShowMouseCursor _returnvalue true)
        (Input|SetInputModeGameandUI _returnvalue (Variables|Default|GetPauseMenuREF) "DoNotLock" false)))))

(event Input|ActionEvents|InputActionJournal
  (params (Key :type Key%20Structure :default "None"))
  (bind _returnvalue (Game|GetPlayerController 0))
  ;[1 1 1] Open Game Journal
  (:Pressed
    (bind _returnvalue_2 (UserInterface|CreateWidget "/Game/w027457k/UI/UITESTS/UI_GameManual.UI_GameManual_C"))
    (UserInterface|Viewport|AddtoViewport _returnvalue_2 0)
    (Game|SetGamePaused true)
    (Input|SetInputModeUIOnly _returnvalue _returnvalue_2 "DoNotLock")
    (Variables|/Script/Engine.PlayerController|SetbShowMouseCursor _returnvalue true)))

(event Input|KeyboardEvents|Z
  (params (Key :type Key%20Structure :default "None"))
  ;[1 0 0] TEST INPUTS
  (:Pressed
    (Class|BPIGM|IIncreaseLight(Message) (Game|GetGameMode) 15)))

(event Input|KeyboardEvents|H
  (params (Key :type Key%20Structure :default "None"))
  ;[1 0 0] TEST INPUTS
  (:Pressed
    (bind _asgm_main (Utilities|Casting|CastToGM_Main (Game|GetGameMode)))
    (Default|GameComplete _asgm_main)))

(fn ConstructionScript)

(fn ChangePostProcessEnabled
  (params (Set%20Enabled :type Boolean))
  (Variables|/Script/Engine.PostProcessComponent|SetbEnabled (Variables|Default|GetGrayPostProcess) Set%20Enabled))

(fn IGetHealth
  (return (Variables|Default|GetHealth)))

(fn IGetHealth
  (return (Variables|Default|GetHealth)))

(fn IGetInv
  (bind _inventory (Default|GetInventory (Variables|Default|GetBPC_Inventory)))
  (return _inventory))

(fn IGetItem
  (params (itemIndex :type Integer))
  (bind _item (Default|GetItem (Variables|Default|GetBPC_Inventory) itemIndex))
  (return _item))

(fn IGetMaxSpeed
  (return (Class|MovementComponent|GetMaxSpeed (Variables|Character|GetCharacterMovement))))

(fn IGetPlayerRef
  (return self))

(fn IGetUI
  (return (Variables|Default|GetplayerUI)))

(fn IIsHoldingItem
  (return (Variables|Default|GetisHolding)))