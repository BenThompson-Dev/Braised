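; Main game mode that starts up the level and relays light and journal changes.
; BeginPlay initialises the player controller, shed and pen manager through interface calls, then, if the pen manager exists, the darkness sphere, StarFruit manager, food spawners and pickups.
; It forwards light increases to the sphere, stores journal pages, enables VSync and quits on Escape.
; A darkness countdown has interface getters, but its timer start and widget creation are disconnected.
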(event Custom|CreateUI
  ;[1 1 1] Create Darkness UI on Delay - l014519j
)

(event Custom|TimerUpdate
  ;[1 1 1] Timer Function and update to UI Progress Bar ( TEMP CAMERA FADE AND QUIT- GAME TO UPDATE AND CHANGE HANDLING DEATH EDIT FROM HERE) - l014519j
  (if (== (Variables|Default|GetSec) 0)
    (if (== (Variables|Default|GetMin) 0)
      (Utilities|FlowControl|Delay 21.0)
      (bind _aspc_player (Utilities|Casting|CastToPC_Player (Game|GetPlayerController 0)))
      (Default|Darkness _aspc_player)
      (else
        (Variables|Default|SetSec 300)))
    (else
      (bind _output_get (Variables|Default|SetSec (- (Variables|Default|GetSec) 1)))
      (bind _output_get_2 (Variables|Default|SetSet%20Percent _output_get))
      (Variables|Default|SetPercent (Math|Conversions|ToFloat(Integer) _output_get_2)))))

(event Custom|InitDarknessBar
  (Utilities|FlowControl|Sequence
    (:then_0
      ;[1 1 1] t014172k -VSync setup
      (bind _returnvalue (Settings|GetGameUserSettings))
      (Class|GameUserSettings|SetVSyncEnabled _returnvalue true)
      (Class|GameUserSettings|ApplySettings _returnvalue true))
    (:then_1
      (CallFunction|CreateUI))))

(event EventBeginPlay
  ;[1 1 1] t014172k - Game mode initialisation chain
  (Class|BPIInit|IInit(Message) (Game|GetPlayerController 0))
  (bind _returnvalue (Actor|GetActorOfClass "/Game/t014172k/Blueprints/BP_Shed.BP_Shed_C"))
  (Utilities|IsValid _returnvalue
    (:Is%20Valid
      (Default|IInit _returnvalue))
    (:Is%20Not%20Valid
      _))
  (bind _returnvalue_2 (Actor|GetActorOfClass "/Game/b014818k/Blueprints/BP_PenManager.BP_PenManager_C"))
  (Utilities|IsValid _returnvalue_2
    (:Is%20Valid
      (Default|IInit _returnvalue_2)
      (bind _returnvalue_3 (Actor|GetActorOfClass "/Game/l014519j/Blueprints/BP_DarknessSphereTest.BP_DarknessSphereTest_C"))
      (bind _output_get (Variables|Default|SetdarknessSphere _returnvalue_3))
      (Class|BPIInit|IInit(Message) _output_get)
      (Default|IInit (Variables|Default|GetBPC_StarFruitManager))
      (bind _outactors (Actor|GetAllActorsOfClass "/Game/b014818k/Blueprints/BP_FoodSpawner.BP_FoodSpawner_C"))
      (for _array_element _outactors
        (Class|BPIInit|IInit(Message) _array_element))
      (bind _outactors_2 (Actor|GetAllActorsOfClass "/Game/t014172k/Blueprints/Items/BP_PickupItem.BP_PickupItem_C"))
      (for _array_element_2 _outactors_2
        (Class|BPIInit|IInit(Message) _array_element_2)))))

(event EventIIncreaseLight
  (params (lightIncreaseAmount :type Integer))
  ;[1 1 1] t014172k - Increases the light amount
  (Class|BPIGM|IIncreaseLight(Message) (Variables|Default|GetdarknessSphere) lightIncreaseAmount))

(event EventISetSpecificJournalPage
  (params (Page :type User%20Widget%20Object%20Reference) (PageNumber :type Integer))
  (bind _returnvalue (- PageNumber 1))
  (bind _journalpages (Variables|Default|GetJournalPages))
  ;[1 1 1] Sets the specific journal page
  (if (> (Utilities|Array|Length _journalpages) _returnvalue)
    (Utilities|Array|AddUnique _journalpages Page)
    (else
      (Utilities|Array|Insert _journalpages Page _returnvalue))))

(event Input|KeyboardEvents|Escape
  (params (Key :type Key%20Structure :default "None"))
  ;[1 1 1] Quit Game - l014519j
  (:Pressed
    (Game|QuitGame 0 "Quit" false)))

(fn ConstructionScript)

(fn IGetJournalPages
  (return 0))

(fn IGetPercent
  (return (Variables|Default|GetPercent)))

(fn IGetSec
  (return (Variables|Default|GetSec)))

(fn IGetTimer
  (return (Variables|Default|GetSet%20Percent)))