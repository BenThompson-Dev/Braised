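; Wood pickup item that extends a parent pickup and can be used on an actor to add wood to its pen inventory.
; Interacting runs the parent logic and, once only, tells the game mode to unlock two sub-pages, the second after a delay.
; Using it sends interface calls to the hit actor to add and check wood, returning the check result.
; Destruction spawns a wood particle burst slightly above it.
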(event EventBeginPlay
  (|CallParentFunction) ; This node is disabled and will not be called.\nDrag off pins to build functionality.
)

(event Collision|EventActorBeginOverlap
  (params (OtherActor :type Actor%20Object%20Reference)))

(event EventTick
  (params (DeltaSeconds :type Float%20%28single-precision%29)))

(event EventIInteract
  (params (playerRef :type Character%20Object%20Reference) (Jakesplayerref :type CH%20Player%20Object%20Reference))
  (|CallParentFunction playerRef 0)
  (Utilities|FlowControl|DoOnce false
    (:Completed
      (Class|BPIGM|IUnlockSubPages(Message) (Game|GetGameMode) "NewEnumerator7" true)
      (Utilities|FlowControl|Delay 6.0)
      (Class|BPIGM|IUnlockSubPages(Message) (Game|GetGameMode) "NewEnumerator12" true))))

(event EventDestroyItem
  (bind _defaultsceneroot (Variables|Default|GetDefaultSceneRoot))
  (bind _returnvalue (Transformation|GetWorldTransform _defaultsceneroot))
  (bind (_location _rotation _scale) (Math|Transform|BreakTransform _returnvalue))
  (bind (_x _y _z) (Math|Vector|BreakVector _location))
  (Game|SpawnActorfromClass "/Game/b014818k/Blueprints/BP_WoodParticleBurst.BP_WoodParticleBurst_C" (Math|Transform|MakeTransform (Math|Vector|MakeVector _x _y (+ _z 3e+01)) _rotation _scale) "Undefined" 0 0)
  (Actor|DestroyActor))

(fn ConstructionScript
  (|CallParentFunction))

(fn UseFunctionality
  (params (hitActor :type Actor%20Object%20Reference))
  ;[1 1 1] t014172k - Tries to add wood to the pen inventory
  (Class|BPIPen|IAddWood(Message) hitActor self)
  (bind _successful (Class|BPIPen|ICheckWood(Message) hitActor))
  (return _successful))