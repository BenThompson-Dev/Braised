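; Pickup item actor that players can add to their inventory, hold and use.
; On BeginPlay it looks up its data in DT_InventoryItems by ItemID.
; Interface calls drive it: interacting passes the item to the player and binds a destroy callback, while holding shrinks it and disables mesh collision.
; Using it line-traces from the player camera and sends any hit actor to UseFunctionality, which here only prints a debug message.
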(event Custom|DestroyItem
  (Actor|DestroyActor))

(event EventIInteract
  (params (playerRef :type Character%20Object%20Reference))
  (bind _playerref (Class|BPIPlayer|IGetPlayerRef(Message) playerRef))
  (EventDispatchers|BindEventtoDestroyItem _playerref (delegate Custom|DestroyItem))
  (Class|BPIPlayer|IAddItem(Message) _playerref (Variables|Default|Getitem) self))

(event EventIHold
  (Development|PrintString "Hello")
  (Transformation|SetActorScale3D "0.250000,0.250000,0.250000")
  (Collision|SetCollisionEnabled (Variables|Default|GetObjectMesh) "NoCollision"))

(event EventBeginPlay
  (bind _itemdata (CallFunction|GetItemData))
  (Variables|Default|Setitem _itemdata))

(fn ConstructionScript)

(fn GetItemData
  ;[1 1 1] Gets each data table row
  (bind _outrownames (DataTable|GetDataTableRowNames "/Game/t014172k/Data/DT_InventoryItems.DT_InventoryItems"))
  (for _array_element _outrownames
    ;[1 1 1] Checks to see if the current data table row has the same ID
    (bind _returnvalue (Utilities|GetDataTableRow "/Game/t014172k/Data/DT_InventoryItems.DT_InventoryItems" _array_element)
      (:then
        (if (== (.itemID (Utilities|Struct|BreakStruct_InventoryItem _returnvalue)) (Variables|Default|GetitemID))
          (return _returnvalue))))))

(fn UseFunctionality
  (params (hitActor :type Actor%20Object%20Reference))
  (Development|PrintString "item used"))

(fn ICanPickup
  (return true))

(fn IUse
  (params (playerCameraRef :type Camera%20Component%20Object%20Reference))
  (bind _returnvalue (Transformation|GetWorldLocation playerCameraRef))
  (bind (_outhit _returnvalue_2) (Collision|LineTraceByChannel _returnvalue (+ _returnvalue (* (Math|Vector|GetForwardVector playerCameraRef) (Variables|Default|GettraceLength))) "TraceTypeQuery2" false (Utilities|Array|MakeArray (Game|Player|GetPlayerPawn 0)) "None"))
  (if _returnvalue_2
    (Development|PrintString (Utilities|GetDisplayName (.HitActor (Collision|BreakHitResult _outhit))))
    (CallFunction|UseFunctionality (.HitActor (Collision|BreakHitResult _outhit)))
    (return true)
    (else
      (Development|PrintString "no objects hit")
      (return false))))