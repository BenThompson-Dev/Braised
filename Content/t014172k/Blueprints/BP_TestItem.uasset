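; BP_TestItem is a test item actor that offers an inventory item to any actor that overlaps its box.
; On BeginPlay, GetItemInfo loops through the DT_InventoryItems rows for the one matching its ItemID and caches it as Item, printing debug messages on mismatches.
; Box overlap passes Item to the other actor through the IAddItemMessage interface call, without destroying itself.
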(event OnComponentBeginOverlap(Box)
  (params (OverlappedComponent :type Primitive%20Component%20Object%20Reference) (OtherActor :type Actor%20Object%20Reference) (OtherComp :type Primitive%20Component%20Object%20Reference) (OtherBodyIndex :type Integer) (bFromSweep :type Boolean) (SweepResult :type Hit%20Result%20Structure%20%28by%20ref%29))
  (Class|BPIPlayer|IAddItem(Message) OtherActor (Variables|Default|Getitem)))

(event EventBeginPlay
  (bind _item (CallFunction|GetItemInfo))
  (Variables|Default|Setitem _item))

(fn ConstructionScript)

(fn GetItemInfo
  ;[1 1 1] Gets each data table row
  (bind _outrownames (DataTable|GetDataTableRowNames "/Game/t014172k/Data/DT_InventoryItems.DT_InventoryItems"))
  (for _array_element _outrownames
    ;[1 1 1] Checks to see if the current data table row has the same ID
    (bind _returnvalue (Utilities|GetDataTableRow "/Game/t014172k/Data/DT_InventoryItems.DT_InventoryItems" _array_element)
      (:then
        (if (== (.itemID (Utilities|Struct|BreakStruct_InventoryItem _returnvalue)) (Variables|Default|GetitemID))
          (return _returnvalue)
          (else
            (Development|PrintString "not correct row"))))))
  (Development|PrintString "item info not found"))