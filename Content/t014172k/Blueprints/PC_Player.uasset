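; Player controller that relays player input to the controlled pawn and handles game-over events.
; IInit caches the pawn and initialises it, then movement, look, jump, sprint, tool interaction, item use and item switching inputs are forwarded to it as interface messages.
; Death from damage or darkness calls RestartGame on the game mode, reached through an interface getter, then opens the game-over map.
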(event Custom|Darkness
  ;[1 1 1] l014519j - Death From Darkness
  (bind _gamemode (Class|BPIGM|IGetGM(Message) (Game|GetGameMode)))
  (Class|GameMode|RestartGame _gamemode)
  (Game|OpenLevel(byName) "GameOverMap"))

(event Custom|Death
  ;[1 1 1] Restarts the game if too much damage is taken - l014519j
  (bind _gamemode (Class|BPIGM|IGetGM(Message) (Game|GetGameMode)))
  (Class|GameMode|RestartGame _gamemode)
  (Game|OpenLevel(byName) "GameOverMap"))

(event EventIInit
  ;[1 1 1] Initialises the player and player controller
  (bind _output_get (Variables|Default|SetplayerPawn (Pawn|GetControlledPawn)))
  (Class|BPIInit|IInit(Message) _output_get))

(event Input|ActionEvents|InputActionJump
  (params (Key :type Key%20Structure :default "None"))
  ;[1 1 1] Player input events
  (:Pressed
    (Class|BPIPlayer|IJump(Message) (Variables|Default|GetplayerPawn))))

(event Input|ActionEvents|InputActionSprint
  (params (Key :type Key%20Structure :default "None"))
  ;[1 1 1] Player input events
  (:Pressed
    (Class|BPIPlayer|ISprint(Message) (Variables|Default|GetplayerPawn) true))
  (:Released
    (Class|BPIPlayer|ISprint(Message) (Variables|Default|GetplayerPawn) false)))

(event Input|ActionEvents|InputActionSetItem
  (params (Key :type Key%20Structure :default "None"))
  (bind _playerpawn (Variables|Default|GetplayerPawn))
  ;[1 1 1] Item switching input
  (:Pressed
    (if (== Key "Two")
      (Class|BPIPlayer|ISetHeldItem(Message) _playerpawn 1)
      (else
        (Class|BPIPlayer|ISetHeldItem(Message) _playerpawn)))))

(event Input|ActionEvents|InputActionInteract
  (params (Key :type Key%20Structure :default "None"))
  (bind _playerpawn (Variables|Default|GetplayerPawn))
  (:Pressed
    (Class|BPIPlayer|IToolInteract(Message) _playerpawn))
  (:Released
    (Class|BPIPlayer|IToolInteractReleased(Message) _playerpawn)))

(event Input|ActionEvents|InputActionUse
  (params (Key :type Key%20Structure :default "None"))
  (:Pressed
    (Class|BPIPlayer|IItemUse(Message) (Variables|Default|GetplayerPawn))))

(event Input|AxisEvents|InputAxisSwapItem
  (params (AxisValue :type Float%20%28single-precision%29))
  ;[1 1 1] Item switching input
  (if (not (Math|Float|NearlyEqual(Float) AxisValue 0.0 0.001))
    (Class|BPIPlayer|ISwapHeldItem(Message) (Variables|Default|GetplayerPawn) (>= AxisValue 0.0))))

(event Input|AxisEvents|InputAxisMoveForward
  (params (AxisValue :type Float%20%28single-precision%29))
  ;[1 1 1] Player input events
  (Class|BPIPlayer|IMoveForward(Message) (Variables|Default|GetplayerPawn) AxisValue))

(event Input|AxisEvents|InputAxisMoveRight
  (params (AxisValue :type Float%20%28single-precision%29))
  ;[1 1 1] Player input events
  (Class|BPIPlayer|IMoveRight(Message) (Variables|Default|GetplayerPawn) AxisValue))

(event Input|AxisEvents|InputAxisTurn
  (params (AxisValue :type Float%20%28single-precision%29))
  ;[1 1 1] Player input events
  (Class|BPIPlayer|ITurn(Message) (Variables|Default|GetplayerPawn) AxisValue))

(event Input|AxisEvents|InputAxisLookUp
  (params (AxisValue :type Float%20%28single-precision%29))
  ;[1 1 1] Player input events
  (Class|BPIPlayer|ILookUp(Message) (Variables|Default|GetplayerPawn) AxisValue))

(fn ConstructionScript)